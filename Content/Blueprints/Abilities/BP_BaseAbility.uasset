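; Base ability actor for a fighting-game character, with empty start, land and animation-end hooks plus helpers for parent movement, states, projectiles and throws.
; The construction script caches hitbox settings from child BP_damagerInfo actors into arrays.
; Montage notifies spawn the current collision set as damagers or grab boxes, mirrored by facing, through server and client events.
; While active, tick handles start, landing, charging and state-triggered ending.
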(event Custom|SoftEnd
  ;[0.3979 0.626 1 1 35] Event Calls
  ;;[1 1 1 1 35] Soft End The active ability
  (CallFunction|WalkOffLedge true)
  (Variables|Default|SetActive false)
  (CallFunction|SetFlip true)
  (CallFunction|SetJump true)
  (CallFunction|SetMovement true)
  (CallFunction|SetCanAttack true)
  (CallFunction|RemoveDamagers)
  (Variables|Default|SetInUse false))

(event Custom|SetMovement
  (params (CanMove :type Boolean))
  ;[0.3979 0.626 1 1 35] Event Calls
  (Variables|/Game/Blueprints/Characters/BP_Fighter.BP_Fighter_C|SetCanMove (Variables|Default|GetParent) CanMove))

(event Custom|PlayAnimation_Server
  (params (Anim%20No :type Integer) (MontageToPlay :type Anim%20Montage%20Object%20Reference))
  ;[0.3979 0.626 1 1 35] Event Calls
  ;;[1 0.9152 0.5198 1 30] PlayAnimations
  (Animation|Montage|PlayMontage (Variables|/Script/Engine.Character|GetMesh (Variables|Default|GetParent)) MontageToPlay
    (:OnBlendOut
      (CallFunction|EndAnim Anim%20No))
    (:OnInterrupted
      (CallFunction|AnimNotifyEnd (Variables|Default|GetDamager) "None" :!label _label))
    (:OnNotifyBegin
      (if (or (Utilities|Name|Equal(Name) (stale Custom|PlayAniamtionClient _notifyname) "None") (Utilities|Set|Contains (Variables|Default|GetAttackContain) (stale Custom|PlayAniamtionClient _notifyname)))
        (Variables|Default|SetDamager true)
        (else
          (Variables|Default|SetDamager false)))
      (CallFunction|AnimNotifyStart (Variables|Default|GetDamager) "None"))
    (:OnNotifyEnd
      (goto _label))))

(event Custom|SetCanAttack
  (params (CanAttack :type Boolean))
  ;[0.3979 0.626 1 1 35] Event Calls
  (Variables|/Game/Blueprints/Characters/BP_Fighter.BP_Fighter_C|SetCanAttack (Variables|Default|GetParent) CanAttack))

(event Custom|StopAllMovement
  ;[0.3979 0.626 1 1 35] Event Calls
  ;;[1 1 1 1 35] Stops Character Movement
  (Components|Movement|StopMovementImmediately (Pawn|GetMovementComponent (Variables|Default|GetParent))))

(event Custom|FreeFall
  ;[0.3979 0.626 1 1 35] Event Calls
  (Variables|/Game/Blueprints/Characters/BP_Fighter.BP_Fighter_C|SetStates (Variables|Default|GetParent) "NewEnumerator20"))

(event Custom|WalkOffLedge
  (params (CanWalkOff :type Boolean))
  ;[0.3979 0.626 1 1 35] Event Calls
  (Variables|/Script/Engine.CharacterMovementComponent|SetbCanWalkOffLedges (Variables|/Script/Engine.Character|GetCharacterMovement (Variables|Default|GetParent)) CanWalkOff))

(event Custom|LandLag
  (params (LandAnimation :type Anim%20Montage%20Object%20Reference) (PlayRate :type Float%20%28single-precision%29) (StartPosition :type Float%20%28single-precision%29) (StartSection :type Name) (AnimNo :type Integer))
  ;[0.3979 0.626 1 1 35] Event Calls
  ;;[0.3265 0.6439 1 1 35] Landing Lag
  (CallFunction|SetFlip false)
  (CallFunction|SetJump false)
  (CallFunction|SetMovement false)
  (Animation|Montage|PlayMontage (Variables|/Script/Engine.Character|GetMesh (Variables|Default|GetParent)) LandAnimation PlayRate StartPosition StartSection
    (:OnBlendOut
      (CallFunction|SetFlip true)
      (CallFunction|SetJump true)
      (CallFunction|SetMovement true)
      (CallFunction|EndAnim AnimNo)
      (Variables|Default|SetLanding false)
      (CallFunction|EndAbility))))

(event Custom|SetFlip
  (params (CanFlip :type Boolean))
  ;[0.3979 0.626 1 1 35] Event Calls
  (Variables|/Game/Blueprints/Characters/BP_Fighter.BP_Fighter_C|SetCanFlip (Variables|Default|GetParent) CanFlip))

(event Custom|SetJump
  (params (CanJump_0 :type Boolean))
  ;[0.3979 0.626 1 1 35] Event Calls
  (Variables|/Game/Blueprints/Characters/BP_Fighter.BP_Fighter_C|SetCanJump_0 (Variables|Default|GetParent) CanJump_0))

(event Custom|ActivateOverAbility
  (params (Ability :type BP%20Base%20Ability%20Object%20Reference))
  ;[0.3979 0.626 1 1 35] Event Calls
  (bind _outactors (Actor|GetAllActorsOfClass "BP_BaseAbility_C"))
  (for _array_element _outactors
    (if (and (== Ability _array_element) (== _array_element (Components|GetOwner (Variables|Default|GetParent))))
      _)))

(event Custom|Throw
  (params (Attack :type Name))
  (bind _parent (Variables|Default|GetParent))
  (bind _attachedto (Variables|/Game/Blueprints/Characters/BP_Fighter.BP_Fighter_C|GetAttachedTo _parent))
  ;[0.3979 0.626 1 1 35] Event Calls
  ;;[1 0.642 0.4696 1 35] Throwing
  (bind _returnvalue (Utilities|GetDataTableRow (Variables|Default|GetAttackData) Attack)
    (:then
      (Default|Hit _attachedto (Variables|/Game/Blueprints/Characters/BP_Fighter.BP_Fighter_C|GetFaceing _parent) (.Damage (Utilities|Struct|BreakST_AttacksStruct _returnvalue)) (.ShildDamage (Utilities|Struct|BreakST_AttacksStruct _returnvalue)) (Math|Float|Truncate (.BaseKnock (Utilities|Struct|BreakST_AttacksStruct _returnvalue))) (.Scale (Utilities|Struct|BreakST_AttacksStruct _returnvalue)) (.Angle (Utilities|Struct|BreakST_AttacksStruct _returnvalue)) (.HitStop (Utilities|Struct|BreakST_AttacksStruct _returnvalue)) (.HitStun (Utilities|Struct|BreakST_AttacksStruct _returnvalue)))
      (Transformation|DetachFromActor _attachedto "KeepWorld" "KeepWorld" "KeepWorld"))))

(event Custom|AddDamagersClient
  (params (Parent :type BP%20Fighter%20Object%20Reference))
  ;[0.3979 0.626 1 1 35] Event Calls
  ;;[1 0.4365 0.4323 1 35] Attach Damage boxes
  (CallFunction|FuncDamageBoxes Parent))

(event Custom|HitStates
  (params (State :type Enum_HitStates%20Enum :default "NewEnumerator0"))
  ;[0.3979 0.626 1 1 35] Event Calls
  (Variables|/Game/Blueprints/Characters/BP_Fighter.BP_Fighter_C|SetHitStates (Variables|Default|GetParent) State))

(event Custom|FlipOnStick
  (bind _parent (Variables|Default|GetParent))
  (bind _parent_2 (Variables|Default|GetParent))
  (bind _capsulecomponent (Variables|/Script/Engine.Character|GetCapsuleComponent _parent_2))
  (bind _leftright (Variables|/Game/Blueprints/Characters/BP_Fighter.BP_Fighter_C|GetLeftRight _parent))
  ;[0.3979 0.626 1 1 35] Event Calls
  ;;[0.59 1 0.814 1 35] Flip Direction at the start of move on stick direction
  (switch Utilities|FlowControl|Switch|SwitchonEnum_faceing (Variables|/Game/Blueprints/Characters/BP_Fighter.BP_Fighter_C|GetFaceing _parent)
    (:NewEnumerator0
      (if (> _leftright 0.0)
        (Transformation|SetActorRotation _parent_2 "0,-90.000000, 0")
        (Variables|/Game/Blueprints/Characters/BP_Fighter.BP_Fighter_C|SetFaceing _parent_2 "NewEnumerator1")
        (Transformation|SetWorldRotation _capsulecomponent "0,90.000000, 0" false false)))
    (:NewEnumerator1
      (if (< _leftright 0.0)
        (Transformation|SetActorRotation _parent_2 "0,90.000000, 0")
        (Variables|/Game/Blueprints/Characters/BP_Fighter.BP_Fighter_C|SetFaceing _parent_2 "NewEnumerator0")
        (Transformation|SetWorldRotation _capsulecomponent "0,-90.000000, 0" false false)))))

(event Custom|Add%20Damagers%20Server
  (params (Parent :type BP%20Fighter%20Object%20Reference))
  ;[0.3979 0.626 1 1 35] Event Calls
  ;;[1 0.4365 0.4323 1 35] Attach Damage boxes
  (CallFunction|FuncDamageBoxes Parent))

(event Custom|CharacterCollsion
  (params (NewType :type ECollisionEnabled%20Enum :default "NoCollision"))
  ;[0.3979 0.626 1 1 35] Event Calls
  (Collision|SetCollisionEnabled (Variables|/Script/Engine.Character|GetCapsuleComponent (Variables|Default|GetParent)) NewType))

(event Custom|ReSheild
  (bind _parent (Variables|Default|GetParent))
  ;[0.3979 0.626 1 1 35] Event Calls
  ;;[1 0.4192 0.9753 1 35] Go back into sheild at end
  (Utilities|FlowControl|Delay 0.01)
  (if (Variables|/Game/Blueprints/Characters/BP_Fighter.BP_Fighter_C|GetShieldButton _parent)
    (Variables|/Game/Blueprints/Characters/BP_Fighter.BP_Fighter_C|SetStates _parent "NewEnumerator12")))

(event Custom|StartParticles
  (params (Attached? :type Boolean) (EmitterTemplate :type Particle%20System%20Object%20Reference) (AttachToComponent :type Scene%20Component%20Object%20Reference) (AttachPointName :type Name) (Location :type Vector) (Rotation :type Rotator) (Scale :type Vector) (LocationType :type EAttachLocation%20Enum :default "KeepRelativeOffset") (bAutoDestroy :type Boolean))
  ;[0.3979 0.626 1 1 35] Event Calls
  (if Attached?
    (Effects|SpawnEmitterAttached EmitterTemplate AttachToComponent AttachPointName Location Rotation Scale LocationType bAutoDestroy)
    (else
      (Effects|SpawnEmitteratLocation EmitterTemplate Location Rotation Scale bAutoDestroy))))

(event Custom|ShootProjectile
  ;[0.3979 0.626 1 1 35] Event Calls
)

(event Custom|Charge
  (params (Chargeing :type Boolean))
  ;[0.3979 0.626 1 1 35] Event Calls
  (Variables|charge|SetChargeing Chargeing))

(event Custom|PlayAnimation
  (params (Anim%20No :type Integer))
  (bind _animations (Variables|Animation|GetAnimations))
  (bind _output (Utilities|Array|Get(acopy) _animations Anim%20No))
  ;[0.3979 0.626 1 1 35] Event Calls
  ;;[1 0.9152 0.5198 1 30] PlayAnimations
  (CallFunction|PlayAnimationServer Anim%20No _output)
  (CallFunction|PlayAniamtionClient Anim%20No _output))

(event Custom|ChangeCollisionSet
  (params (CollisionSetInex :type Integer))
  ;[0.3979 0.626 1 1 35] Event Calls
  (bind _output_get (Variables|Collisions|SetCollisionSetIndex (+ 1 (Variables|Collisions|GetCollisionSetIndex))))
  (Variables|Collisions|SetCollisionSet (Utilities|Array|Get(acopy) (Variables|Collisions|GetCollisionSetArray) _output_get)))

(event Custom|SetAttackStage
  (params (AttackStage :type Integer))
  ;[0.3979 0.626 1 1 35] Event Calls
  (Variables|Default|SetAttackStage AttackStage))

(event Custom|FullbodyLedge
  (params (FullBodyLedgeGrab :type Boolean))
  ;[0.3979 0.626 1 1 35] Event Calls
  (Variables|/Game/Blueprints/Characters/BP_Fighter.BP_Fighter_C|SetFullBodyLedgeGrab (Variables|Default|GetParent) FullBodyLedgeGrab))

(event Custom|AbilityStart
  ;[0.3979 0.626 1 1 35] Event Calls
)

(event Custom|EndAnim
  (params (AnimNo :type Integer))
  ;[0.3979 0.626 1 1 35] Event Calls
)

(event Custom|DodgeDelay
  ;[0.3979 0.626 1 1 35] Event Calls
  (Default|DodgeDelayEvent (Variables|Default|GetParent)))

(event Custom|AnimNotifyEnd
  (params (Damager :type Boolean) (NoteName :type Name))
  ;[0.3979 0.626 1 1 35] Event Calls
  (if Damager
    (CallFunction|RemoveDamagers)))

(event Custom|RemoveDamagers
  ;[0.3979 0.626 1 1 35] Event Calls
  ;;[0.8782 1 0.4333 1 35] Remove Damagers
  (bind _outactors (Actor|GetAllActorsOfClass "/Game/Blueprints/PlayerObjects/BP_damager.BP_damager_C"))
  (for _array_element _outactors
    (if (== (Variables|/Game/Blueprints/PlayerObjects/BP_damager.BP_damager_C|GetParent _array_element) (Variables|Default|GetParent))
      (Actor|DestroyActor _array_element))))

(event Custom|TickRep
  (bind _parent (Variables|Default|GetParent))
  (bind _states (Variables|/Game/Blueprints/Characters/BP_Fighter.BP_Fighter_C|GetStates _parent))
  ;[1 1 1 1 35] Tick
  (if (Variables|Default|GetActive)
    (Utilities|FlowControl|Sequence
      (:then_0
        (if (not (Variables|Default|GetInUse))
          (CallFunction|AbilityStart)
          (Variables|Default|SetInUse true)))
      (:then_1
        (if (Variables|/Game/Blueprints/Characters/BP_Fighter.BP_Fighter_C|GetLanded _parent)
          (Utilities|FlowControl|DoOnce false :!label _label
            (:Completed
              (Variables|Default|SetLanding true)
              (CallFunction|Land)))
          (else
            (goto _label Reset))))
      (:then_2
        (CallFunction|FuncCharaging))
      (:then_3
        (if (or (Utilities|Enum|Equal(Enum) _states "NewEnumerator9") (Utilities|Enum|Equal(Enum) _states "NewEnumerator5"))
          (CallFunction|EndAbility)))
      (:then_4
        (if (Utilities|Enum|Equal(Enum) _states "NewEnumerator8")
          _)))))

(event Custom|EndAllNonChargedAbilities
  (params (Caller :type BP%20Base%20Ability%20Object%20Reference))
  ;[0.3979 0.626 1 1 35] Event Calls
  (Default|EndAllNonChargedAbilities (Variables|/Game/Blueprints/Characters/BP_Fighter.BP_Fighter_C|GetAbility (Variables|Default|GetParent)) Caller))

(event Custom|SetGravity
  (params (Settings :type Enum_EnbaleDisable%20Enum :default "NewEnumerator0") (CustomValue :type Float%20%28single-precision%29))
  (bind _parent (Variables|Default|GetParent))
  (bind _parent_2 (Variables|Default|GetParent))
  (bind _charactermovement (Variables|/Script/Engine.Character|GetCharacterMovement _parent_2))
  ;[0.3979 0.626 1 1 35] Event Calls
  (switch Utilities|FlowControl|Switch|SwitchonEnum_EnbaleDisable Settings
    (:NewEnumerator0
      (Variables|/Script/Engine.CharacterMovementComponent|SetGravityScale (Variables|/Script/Engine.Character|GetCharacterMovement _parent) (Variables|/Game/Blueprints/PlayerObjects/BPC_BP_CharacterStats.BPC_BP_CharacterStats_C|GetDefultGravityScale (Variables|/Game/Blueprints/Characters/BP_Fighter.BP_Fighter_C|GetCharacterStats _parent))))
    (:NewEnumerator1
      (Variables|/Script/Engine.CharacterMovementComponent|SetGravityScale _charactermovement 0.0))
    (:NewEnumerator2
      (Variables|/Script/Engine.CharacterMovementComponent|SetGravityScale _charactermovement CustomValue))))

(event Custom|AnimNotifyStart
  (params (Damager :type Boolean) (NoteName :type Name))
  ;[0.3979 0.626 1 1 35] Event Calls
  (if Damager
    (CallFunction|ActivateDamagers)
    (elif (Utilities|Name|Equal(Name) NoteName "ChangeSet")
      (CallFunction|ChangeCollisionSet))))

(event Custom|CameraZoom
  (params (Zoom%20Amount :type Float%20%28single-precision%29) (Duration :type Float%20%28single-precision%29))
  ;[0.3979 0.626 1 1 35] Event Calls
)

(event Custom|Reset
  ;[0.3979 0.626 1 1 35] Event Calls
  ;;[1 1 1 1 35] Resets Values of ability
  (Variables|charge|SetChargeLevel 0.0)
  (Variables|charge|SetChargeRatio 0.0)
  (Variables|charge|SetChargeLevel 0.0)
  (Variables|charge|SetChargeing false)
  (Variables|charge|SetCharged false)
  (Variables|Default|SetInUse false)
  (Variables|Animation|SetAnimNo 1)
  (Variables|Collisions|SetCollisionSet 1)
  (Variables|Default|SetActivateCollision false)
  (CallFunction|WalkOffLedge true)
  (Variables|Collisions|SetCollisionSetIndex 0))

(event Custom|GetCollisionInfo
  ;[0.3979 0.626 1 1 35] Event Calls
)

(event Custom|SpawnProjectile
  (params (Projectile :type BP%20Projectile%20Base%20Class%20Reference) (Transform :type Transform) (LifetIme :type Float%20%28single-precision%29) (YSpeed :type Float%20%28single-precision%29) (ZSpeed :type Float%20%28single-precision%29) (Gravity :type Float%20%28single-precision%29) (AttackName :type Name))
  (bind _parent (Variables|Default|GetParent))
  ;[0.3979 0.626 1 1 35] Event Calls
  ;;[0.4167 0.4167 0.4167 1 35] SpwanProjectile
  (Game|SpawnActorfromClass Projectile Transform "Undefined" _parent (Variables|charge|GetChargeRatio) LifetIme YSpeed ZSpeed Gravity _parent (Variables|/Game/Blueprints/Characters/BP_Fighter.BP_Fighter_C|GetFaceing _parent) AttackName _parent))

(event Custom|CustomEvent_0
  ;[0.3979 0.626 1 1 35] Event Calls
)

(event Custom|Land
  ;[0.3979 0.626 1 1 35] Event Calls
)

(event Custom|EndAbility
  (bind _parent (Variables|Default|GetParent))
  ;[0.3979 0.626 1 1 35] Event Calls
  ;;[1 1 1 1 35] End The active ability
  (CallFunction|WalkOffLedge true)
  (Variables|Default|SetActive false)
  (CallFunction|SetFlip true)
  (CallFunction|SetJump true)
  (CallFunction|SetMovement true)
  (CallFunction|CharacterCollsion "QueryAndPhysics")
  (CallFunction|FullbodyLedge false)
  (if (AI|Components|NavMovement|IsFalling (Pawn|GetMovementComponent (Variables|Default|GetParent)))
    (Variables|/Game/Blueprints/Characters/BP_Fighter.BP_Fighter_C|SetStates _parent "NewEnumerator4")
    (else
      (Variables|/Game/Blueprints/Characters/BP_Fighter.BP_Fighter_C|SetStates _parent "NewEnumerator0")))
  (Variables|/Game/Blueprints/Characters/BP_Fighter.BP_Fighter_C|SetAbilityType _parent "NewEnumerator0")
  (Variables|/Game/Blueprints/Characters/BP_Fighter.BP_Fighter_C|SetAttacks _parent "NewEnumerator27")
  (Variables|Default|SetInUse false))

(event Custom|Activate%20Damagers
  (bind _parent (Variables|Default|GetParent))
  ;[0.3979 0.626 1 1 35] Event Calls
  ;;[1 0.4365 0.4323 1 35] Attach Damage boxes
  (Networking|SwitchHasAuthority
    (:Authority
      (CallFunction|AddDamagersServer _parent))
    (:Remote
      (CallFunction|AddDamagersClient _parent))))

(event Custom|PlayAniamtionClient
  (params (Anim%20No :type Integer) (MontageToPlay :type Anim%20Montage%20Object%20Reference))
  ;[0.3979 0.626 1 1 35] Event Calls
  ;;[1 0.9152 0.5198 1 30] PlayAnimations
  (bind _notifyname (Animation|Montage|PlayMontage (Variables|/Script/Engine.Character|GetMesh (Variables|Default|GetParent)) MontageToPlay)
    (:OnBlendOut
      (CallFunction|EndAnim Anim%20No))
    (:OnInterrupted
      (CallFunction|AnimNotifyEnd (Variables|Default|GetDamager) "None" :!label _label))
    (:OnNotifyBegin
      (if (or (Utilities|Name|Equal(Name) _notifyname "None") (Utilities|Set|Contains (Variables|Default|GetAttackContain) _notifyname))
        (Variables|Default|SetDamager true)
        (else
          (Variables|Default|SetDamager false)))
      (CallFunction|AnimNotifyStart (Variables|Default|GetDamager) "None"))
    (:OnNotifyEnd
      (goto _label))))

(event EventBeginPlay
  ;[0.3979 0.626 1 1 35] Event Calls
  (Components|DestroyComponent (Variables|Default|GetSkeletalMesh))
  (Variables|Default|SetAttackData (Variables|/Game/Blueprints/Characters/BP_Fighter.BP_Fighter_C|GetAttackDataTable (Variables|Default|GetParent))))

(event EventTick
  (params (DeltaSeconds :type Float%20%28single-precision%29))
  ;[1 1 1 1 35] Tick
  (CallFunction|TickRep)
  (Utilities|DebugAbilityCall 0 false))

(fn ConstructionScript
  ;[1 0.6802 0.3462 1 30] Get All Damage Info boxes
  (for (_array_element _array_index) (Actor|GetAllChildActors true)
    (bind _asbp_damager_info (Utilities|Casting|CastToBP_damagerInfo _array_element))
    (Utilities|Array|SetArrayElem (Variables|Default|GetchildDamagers) _array_index _asbp_damager_info true))
  ;[0.5452 0.8477 1 1 30] Get all hitbox information
  (for (_array_element_2 _array_index_2) (Variables|Default|GetchildDamagers)
    (Variables|Default|SetNewVar_0 (Variables|/Game/Blueprints/PlayerObjects/BP_damagerInfo.BP_damagerInfo_C|GetLocation+ _array_element_2))
    (Utilities|Array|SetArrayElem (Variables|Collisions|GetCollisionBoxTransforms) _array_index_2 (Math|Transform|MakeTransform (Utilities|Array|Get(acopy) (Variables|Collisions|GetAttackLocations) _array_index_2) (Variables|/Game/Blueprints/PlayerObjects/BP_damagerInfo.BP_damagerInfo_C|GetRotation _array_element_2) (Variables|/Game/Blueprints/PlayerObjects/BP_damagerInfo.BP_damagerInfo_C|GetScale _array_element_2)) true)
    (Utilities|Array|SetArrayElem (Variables|Collisions|GetAttacks) _array_index_2 (Variables|/Game/Blueprints/PlayerObjects/BP_damagerInfo.BP_damagerInfo_C|GetAttack _array_element_2) true)
    (Utilities|Array|SetArrayElem (Variables|Collisions|GetCollisionShape) _array_index_2 (Variables|/Game/Blueprints/PlayerObjects/BP_damagerInfo.BP_damagerInfo_C|GetCollisionShape _array_element_2) true)
    (Utilities|Array|SetArrayElem (Variables|Collisions|GetCollisionType) _array_index_2 (Variables|/Game/Blueprints/PlayerObjects/BP_damagerInfo.BP_damagerInfo_C|GetType _array_element_2) true)
    (Utilities|Array|SetArrayElem (Variables|Collisions|GetCollisionSockets) _array_index_2 (Variables|/Game/Blueprints/PlayerObjects/BP_damagerInfo.BP_damagerInfo_C|GetSocket _array_element_2) true)
    (Utilities|Array|SetArrayElem (Variables|Collisions|GetCollisionSets) _array_index_2 (Variables|/Game/Blueprints/PlayerObjects/BP_damagerInfo.BP_damagerInfo_C|GetSetNo _array_element_2) true)
    (Utilities|Array|SetArrayElem (Variables|Collisions|GetHitSound) _array_index_2 (Variables|/Game/Blueprints/PlayerObjects/BP_damagerInfo.BP_damagerInfo_C|GetHitSound _array_element_2) true)
    (Utilities|Array|SetArrayElem (Variables|Collisions|GetHitParticel) _array_index_2 (Variables|/Game/Blueprints/PlayerObjects/BP_damagerInfo.BP_damagerInfo_C|GetHitParticel _array_element_2) true)
    (Utilities|Array|SetArrayElem (Variables|Collisions|GetGrabBoxes) _array_index_2 (Variables|/Game/Blueprints/PlayerObjects/BP_damagerInfo.BP_damagerInfo_C|GetGrabBox _array_element_2) true)))

(fn FuncCharaging
  (if (Variables|charge|GetChargeing)
    (Variables|charge|SetChargeLevel (+ (Variables|charge|GetChargeLevel) (Variables|charge|GetChargeRate)))
    (Variables|charge|SetChargeRatio (/ (Variables|charge|GetChargeMax) (Variables|charge|GetChargeLevel)))
    (if (>= (Variables|charge|GetChargeLevel) (Variables|charge|GetChargeMax))
      (Variables|charge|SetChargeLevel (Variables|charge|GetChargeMax))
      (Variables|charge|SetCharged true))))

(fn FuncSetBoxTransform'
  (params (Dimension%201 :type Integer))
  (bind _collisionboxtransforms (Variables|Collisions|GetCollisionBoxTransforms))
  (bind _parent (Variables|Default|GetParent))
  (bind _returnvalue (Transformation|GetActorTransform _parent))
  (bind _output (Utilities|Array|Get(acopy) _collisionboxtransforms Dimension%201))
  (bind _mesh (Variables|/Script/Engine.Character|GetMesh _parent))
  (bind _scale (Math|Transform|BreakTransform _returnvalue))
  (bind _returnvalue_2 (Transformation|GetSocketLocation _mesh "roorSocket"))
  (bind (_location _rotation _scale_2) (Math|Transform|BreakTransform _output))
  (bind (_x _y _z) (Math|Vector|BreakVector _location))
  (bind _returnvalue_3 (* _scale_2 _scale))
  (switch Utilities|FlowControl|Switch|SwitchonEnum_faceing (Variables|/Game/Blueprints/Characters/BP_Fighter.BP_Fighter_C|GetFaceing (Variables|Default|GetParent))
    (:NewEnumerator0
      (Utilities|Array|SetArrayElem (Variables|Default|GetBoxTransforms) Dimension%201 (Math|Transform|MakeTransform (+ _location _returnvalue_2) _rotation _returnvalue_3) true))
    (:NewEnumerator1
      (Utilities|Array|SetArrayElem (Variables|Default|GetBoxTransforms) Dimension%201 (Math|Transform|MakeTransform (+ _returnvalue_2 (Math|Vector|MakeVector _x (* _y -1.0) _z)) _rotation _returnvalue_3) true)))
  (return))

(fn FuncDamageBoxes
  (params (Parent :type BP%20Fighter%20Object%20Reference))
  (for (_ _array_index) (Variables|Default|GetchildDamagers)
    (if (== (Utilities|Array|Get(acopy) (Variables|Collisions|GetCollisionSets) _array_index) (Variables|Collisions|GetCollisionSet))
      ;[0.4688 0.04249 0.1128 1 30] HitBox
      (CallFunction|FuncSetBoxTransform' _array_index)
      (if (not (Utilities|Array|Get(acopy) (Variables|Collisions|GetGrabBoxes) (.Index (Utilities|GetHitPropities _array_index))))
        (bind _returnvalue (Game|SpawnActorfromClass "/Game/Blueprints/PlayerObjects/BP_damager.BP_damager_C" (Utilities|Array|Get(acopy) (Variables|Default|GetBoxTransforms) (.Index (Utilities|GetHitPropities _array_index))) "AlwaysSpawn" 0 Parent (.Collision (Utilities|GetHitPropities _array_index)) (.Shape (Utilities|GetHitPropities _array_index)) (.Priority (Utilities|GetHitPropities _array_index)) (.Socket (Utilities|GetHitPropities _array_index)) (.Faceing (Utilities|GetHitPropities _array_index)) (.FX (Utilities|GetHitPropities _array_index)) (.Sound (Utilities|GetHitPropities _array_index)) (.Attack (Utilities|GetHitPropities _array_index)) 0))
        (bind _output_get (Variables|Collisions|SetHitBox _returnvalue))
        (Utilities|IsValid _output_get
          (:Is%20Valid
            (Transformation|AttachActorToActor _returnvalue (Variables|Default|GetParent) "None" "KeepWorld" "KeepWorld" "KeepWorld" true)))
        (else
          ;[0.2562 0.541 1 0.708 30] GrabBox
          (bind _returnvalue_2 (Game|SpawnActorfromClass "/Game/Blueprints/PlayerObjects/BP_GrabBox.BP_GrabBox_C" (Utilities|Array|Get(acopy) (Variables|Default|GetBoxTransforms) (.Index (Utilities|GetHitPropities _array_index))) "AlwaysSpawn" 0 Parent (.Shape (Utilities|GetHitPropities _array_index)) (.Socket (Utilities|GetHitPropities _array_index)) (.Faceing (Utilities|GetHitPropities _array_index)) (.FX (Utilities|GetHitPropities _array_index)) (.Sound (Utilities|GetHitPropities _array_index)) 0))
          (Utilities|IsValid _returnvalue_2
            (:Is%20Valid
              (Transformation|AttachActorToActor (Variables|Default|GetParent) "None" "KeepWorld" "KeepWorld" "KeepWorld" true))))))))