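; BP_proto_AirForward is a Fighter ability Blueprint, apparently a prototype forward aerial move.
; On start it disables movement, flipping and jumping, then plays animation 0.
; When the animation ends it ends the ability unless Landing is set.
; Landing triggers LandLag with a sped-up neutral-air landing montage rather than one named for forward air.
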(event EventBeginPlay
  (|CallParentFunction))

(event Collision|EventActorBeginOverlap
  (params (OtherActor :type Actor%20Object%20Reference)))

(event EventLand
  (CallFunction|LandLag "/Game/Assets/Characters/Fighter/Animations/AM_nuteralAir01Land_Montage.AM_nuteralAir01Land_Montage" 1.3 0.0 "None"))

(event EventTick
  (params (DeltaSeconds :type Float%20%28single-precision%29))
  (|CallParentFunction DeltaSeconds))

(event EventEndAnim
  (params (AnimNo :type Integer))
  (if (not (Variables|Default|GetLanding))
    (CallFunction|EndAbility)))

(event EventAbilityStart
  (CallFunction|SetMovement false)
  (CallFunction|SetFlip false)
  (CallFunction|SetJump false)
  (CallFunction|PlayAnimation))

(fn ConstructionScript
  (|CallParentFunction))