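; Fighter up-air attack ability, apparently a prototype, built on a shared ability parent.
; On start it locks movement, flipping and jumping, then plays its first animation.
; The ability ends when the animation finishes unless the character is landing.
; Landing instead triggers landing lag with a sped-up neutral-air landing montage.
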(event EventLand
  (CallFunction|LandLag "/Game/Assets/Characters/Fighter/Animations/AM_nuteralAir01Land_Montage.AM_nuteralAir01Land_Montage" 1.3 0.0 "None"))

(event EventEndAnim
  (params (AnimNo :type Integer))
  (if (not (Variables|Default|GetLanding))
    (CallFunction|EndAbility)))

(event EventAbilityStart
  (CallFunction|SetMovement false)
  (CallFunction|SetFlip false)
  (CallFunction|SetJump false)
  (CallFunction|PlayAnimation))

(fn ConstructionScript
  (|CallParentFunction))