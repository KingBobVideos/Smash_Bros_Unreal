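; Prototype fighter ability for an air dodge, either directional or in place.
; On start it locks movement, flip and jump, plays the animation and switches the owner's hit state for a brief window.
; With stick input it disables gravity and launches along that angle, then restores gravity, halting and changing the owner's state if still airborne.
; Animation end or landing ends the ability, with landing adding lag through a montage.
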(event EventBeginPlay
  (|CallParentFunction) ; This node is disabled and will not be called.\nDrag off pins to build functionality.
)

(event Collision|EventActorBeginOverlap
  (params (OtherActor :type Actor%20Object%20Reference)))

(event EventLand
  (CallFunction|LandLag "/Game/Assets/Characters/Fighter/Animations/A_Land_01_Montage.A_Land_01_Montage" 2.0 0.0 "None")
  (CallFunction|EndAbility))

(event EventTick
  (params (DeltaSeconds :type Float%20%28single-precision%29))
  (|CallParentFunction DeltaSeconds) ; This node is disabled and will not be called.\nDrag off pins to build functionality.
)

(event EventEndAnim
  (params (AnimNo :type Integer))
  (CallFunction|HitStates "NewEnumerator0")
  (CallFunction|EndAbility))

(event EventAbilityStart
  (bind _parent (Variables|Default|GetParent))
  (bind _parent_2 (Variables|Default|GetParent))
  (bind _parent_3 (Variables|Default|GetParent))
  (bind _parent_4 (Variables|Default|GetParent))
  (bind _updown (Variables|/Game/Blueprints/Characters/BP_Fighter.BP_Fighter_C|GetUpDown _parent))
  (bind _leftright (Variables|/Game/Blueprints/Characters/BP_Fighter.BP_Fighter_C|GetLeftRight _parent))
  (bind _returnvalue (Class|KismetMathLibrary|DegAtan2 _leftright _updown))
  (bind _returnvalue_2 (Math|Rotator|MakeRotator _returnvalue 0.0 0.0))
  (bind _returnvalue_3 (Math|Vector|GetUpVector _returnvalue_2))
  (bind _returnvalue_4 (Math|Vector|Normalize _returnvalue_3))
  (bind _returnvalue_5 (* _returnvalue_4 1e+03))
  (bind (_x _y _z) (Math|Vector|BreakVector _returnvalue_5))
  (CallFunction|HitStates "NewEnumerator1")
  (CallFunction|SetMovement false)
  (CallFunction|SetFlip false)
  (CallFunction|SetJump false)
  (CallFunction|PlayAnimation)
  (Variables|/Game/Blueprints/Characters/BP_Fighter.BP_Fighter_C|SetHitStates _parent "NewEnumerator1")
  (if (or (!= _leftright 0.0) (!= _updown 0.0))
    (Default|FuncGravity _parent false)
    (Character|LaunchCharacter _parent_3 (Math|Vector|MakeVector _x (* _y -1.0) _z) true true)
    (Utilities|FlowControl|Delay 0.3)
    (if (AI|Components|NavMovement|IsFalling (Pawn|GetMovementComponent _parent_3))
      (Components|Movement|StopMovementImmediately (Variables|/Script/Engine.Character|GetCharacterMovement _parent_3))
      (Variables|/Game/Blueprints/Characters/BP_Fighter.BP_Fighter_C|SetHitStates _parent_4 "NewEnumerator0")
      (Default|FuncGravity _parent_4 true)
      (Variables|/Game/Blueprints/Characters/BP_Fighter.BP_Fighter_C|SetStates _parent_4 "NewEnumerator20")
      (else
        (Variables|/Game/Blueprints/Characters/BP_Fighter.BP_Fighter_C|SetHitStates _parent_2 "NewEnumerator0")
        (Default|FuncGravity _parent_2 true)))
    (else
      (Utilities|FlowControl|Delay 0.2)
      (Variables|/Game/Blueprints/Characters/BP_Fighter.BP_Fighter_C|SetHitStates (Variables|Default|GetParent) "NewEnumerator0"))))

(fn ConstructionScript
  (|CallParentFunction))