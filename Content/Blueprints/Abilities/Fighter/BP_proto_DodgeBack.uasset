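; Prototype fighter ability Blueprint for a backward dodge.
; On start it changes the hit state, disables movement, flipping, jumping and walking off ledges, then plays its animation.
; When the animation ends it switches to the other hit state, ends the ability, calls ReSheild and triggers the dodge delay.
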(event EventEndAnim
  (params (AnimNo :type Integer))
  (CallFunction|HitStates "NewEnumerator0")
  (CallFunction|EndAbility)
  (CallFunction|ReSheild)
  (CallFunction|DodgeDelay))

(event EventAbilityStart
  (CallFunction|HitStates "NewEnumerator1")
  (CallFunction|SetMovement false)
  (CallFunction|SetFlip false)
  (CallFunction|SetJump false)
  (CallFunction|PlayAnimation)
  (CallFunction|WalkOffLedge false))

(fn ConstructionScript
  (|CallParentFunction))