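; Prototype forward dodge ability for the Fighter, built on functions it calls but does not define.
; On start it switches the hit state, disables movement, flipping, jumping and walking off ledges, and plays its animation.
; When the animation ends it restores the other hit state, ends the ability, then calls the re-shield and dodge delay functions.
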(event EventBeginPlay
  (|CallParentFunction) ; This node is disabled and will not be called.\nDrag off pins to build functionality.
)

(event Collision|EventActorBeginOverlap
  (params (OtherActor :type Actor%20Object%20Reference)))

(event EventTick
  (params (DeltaSeconds :type Float%20%28single-precision%29))
  (|CallParentFunction DeltaSeconds) ; This node is disabled and will not be called.\nDrag off pins to build functionality.
)

(event EventEndAnim
  (params (AnimNo :type Integer))
  (CallFunction|HitStates "NewEnumerator0")
  (CallFunction|EndAbility)
  (CallFunction|ReSheild)
  (CallFunction|DodgeDelay))

(event EventAbilityStart
  (CallFunction|HitStates "NewEnumerator1")
  (CallFunction|SetMovement false)
  (CallFunction|SetFlip false)
  (CallFunction|SetJump false)
  (CallFunction|PlayAnimation)
  (CallFunction|WalkOffLedge false))

(fn ConstructionScript
  (|CallParentFunction))