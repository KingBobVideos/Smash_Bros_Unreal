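; A fighter grab ability prototype that locks the character in place and plays a grab animation.
; On start it disables movement, flipping and jumping, then plays the first animation.
; When the animation ends, a holding check either soft-ends the ability while held or ends it fully otherwise.
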(event EventEndAnim
  (params (AnimNo :type Integer))
  (Utilities|Holding (Variables|Default|GetParent)
    (:Holding
      (CallFunction|SoftEnd))
    (:notHold
      (CallFunction|EndAbility))))

(event EventAbilityStart
  (CallFunction|SetMovement false)
  (CallFunction|SetFlip false)
  (CallFunction|SetJump false)
  (CallFunction|PlayAnimation))

(fn ConstructionScript
  (|CallParentFunction))