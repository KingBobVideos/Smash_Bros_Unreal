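; Prototype neutral attack ability for the Fighter that plays a three-stage combo.
; On start it disables movement, flipping and jumping, then plays the current stage's animation and advances AttackStage, wrapping after the last.
; The second and third stages also call ActivateOverAbility.
; When an animation ends, it ends the ability and, after a short delay, resets the combo if the stage has not advanced.
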(event EventEndAnim
  (params (AnimNo :type Integer))
  (CallFunction|EndAbility)
  (Utilities|FlowControl|Delay 0.2)
  (if (== AnimNo (- (Variables|Default|GetAttackStage) 1))
    (CallFunction|SetAttackStage)))

(event EventAbilityStart
  (CallFunction|SetMovement false)
  (CallFunction|SetFlip false)
  (CallFunction|SetJump false)
  (switch int (Variables|Default|GetAttackStage)
    (:0
      (CallFunction|PlayAnimation)
      (CallFunction|SetAttackStage 1))
    (:1
      (CallFunction|ActivateOverAbility)
      (CallFunction|PlayAnimation 1)
      (CallFunction|SetAttackStage 2))
    (:2
      (CallFunction|ActivateOverAbility)
      (CallFunction|PlayAnimation 2)
      (CallFunction|SetAttackStage))))

(fn ConstructionScript
  (|CallParentFunction))