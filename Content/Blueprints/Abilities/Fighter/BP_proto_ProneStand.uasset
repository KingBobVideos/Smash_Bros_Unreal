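; Fighter ability prototype that, going by its name, stands a character up from a prone state.
; On start it disables movement, flipping and jumping, then plays one of two animations depending on whether the parent's Direction is Up or Down.
; The ability ends when the animation end event fires.
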(event EventEndAnim
  (params (AnimNo :type Integer))
  (CallFunction|EndAbility))

(event EventAbilityStart
  (CallFunction|SetMovement false)
  (CallFunction|SetFlip false)
  (CallFunction|SetJump false)
  (switch Utilities|FlowControl|Switch|SwitchonEnum_Direction (Variables|/Game/Blueprints/Characters/BP_Fighter.BP_Fighter_C|GetDirection (Variables|Default|GetParent))
    (:NewEnumerator2
      (CallFunction|PlayAnimation))
    (:NewEnumerator3
      (CallFunction|PlayAnimation 1))))

(fn ConstructionScript
  (|CallParentFunction))