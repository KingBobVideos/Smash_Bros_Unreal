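; Prototype fighter ability Blueprint for a chargeable up smash attack, built on a parent ability class.
; On start it begins charging, disables movement, flipping and jumping, and plays the charge animation.
; Tick polls the parent's attack condition and switches to the attack animation when the input is not pressed.
; The charge animation's end also forces that release, and the attack animation's end finishes the ability.
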(event EventTick
  (params (DeltaSeconds :type Float%20%28single-precision%29))
  (|CallParentFunction DeltaSeconds)
  (Utilities|AttackCondition (Variables|Default|GetParent) (Variables|Default|GetChargeing)
    (:NotPressed
      (CallFunction|PlayAnimation 1)
      (CallFunction|Charge false))))

(event EventEndAnim
  (params (AnimNo :type Integer))
  (switch int AnimNo
    (:0
      (CallFunction|PlayAnimation 1)
      (CallFunction|Charge false))
    (:1
      (CallFunction|EndAbility))))

(event EventAbilityStart
  (CallFunction|Charge true)
  (CallFunction|SetMovement false)
  (CallFunction|SetFlip false)
  (CallFunction|SetJump false)
  (CallFunction|PlayAnimation))

(fn ConstructionScript
  (|CallParentFunction))