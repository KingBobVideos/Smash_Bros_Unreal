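; Prototype down-special ability for a fighter: a rise or hover followed by a fast downward slam, with flip and jump disabled.
; In air it halts movement and changes gravity; on the ground it launches a short hop.
; When the opening animation ends, it switches gravity again, launches straight down and loops the fall animation.
; Tick ends the ability on landing and restores flip and jump, while a Land event applies montage-driven landing lag.
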(event Custom|Fall
  (CallFunction|SetGravity "NewEnumerator0" 0.0)
  (CallFunction|PlayAnimation 1)
  (Default|Launch (Variables|Default|GetParent) "0,0.000000,-2000.000000" true true))

(event EventTick
  (params (DeltaSeconds :type Float%20%28single-precision%29))
  (|CallParentFunction DeltaSeconds)
  (if (Variables|Default|GetActive)
    (if (Variables|/Game/Blueprints/Characters/BP_Fighter.BP_Fighter_C|GetLanded (Variables|Default|GetParent))
      (CallFunction|SetFlip true)
      (CallFunction|SetJump true)
      (CallFunction|EndAbility))))

(event EventAbilityStart
  (CallFunction|SetFlip false)
  (CallFunction|SetJump false)
  (Utilities|InAir? (Variables|Default|GetParent)
    (:Air
      (CallFunction|PlayAnimation)
      (CallFunction|StopAllMovement)
      (CallFunction|SetGravity "NewEnumerator1" 0.0))
    (:Ground
      (CallFunction|PlayAnimation)
      (Default|Launch (Variables|Default|GetParent) "0,0.000000,300.000000" true true))))

(event EventEndAnim
  (params (AnimNo :type Integer))
  (switch int AnimNo
    (:0
      (CallFunction|Fall))
    (:1
      (CallFunction|PlayAnimation 1))))

(event EventLand
  (CallFunction|LandLag "/Game/Assets/Characters/Fighter/Animations/AM_specialDown_land_Montage.AM_specialDown_land_Montage" 1.0 0.0 "None" 2))

(fn ConstructionScript
  (|CallParentFunction))