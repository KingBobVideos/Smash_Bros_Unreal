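; Prototype neutral special ability for a fighter that fires a projectile.
; On start it locks movement, flip and jump, then plays its animation, with an airborne variant that stops momentum, launches the fighter upward and briefly overrides gravity.
; The damager activation event spawns a short-lived projectile at the owner's capsule transform under an attack name.
; The ability ends when the animation ends.
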(event EventEndAnim
  (params (AnimNo :type Integer))
  (CallFunction|EndAbility))

(event EventAbilityStart
  (bind _parent (Variables|Default|GetParent))
  (CallFunction|SetMovement false)
  (CallFunction|SetFlip false)
  (CallFunction|SetJump false)
  (Utilities|InAir? _parent
    (:Air
      (CallFunction|StopAllMovement)
      (CallFunction|SetGravity "NewEnumerator1" 0.0)
      (Default|Launch _parent "0,0.000000,300.000000" true true)
      (CallFunction|PlayAnimation)
      (Utilities|FlowControl|Delay 0.2)
      (CallFunction|SetGravity "NewEnumerator0" 0.0))
    (:Ground
      (CallFunction|PlayAnimation))))

(event EventActivateDamagers
  (CallFunction|SpawnProjectile "/Game/Blueprints/Projectiles/BP_projectile01.BP_projectile01_C" (Transformation|GetWorldTransform (Variables|/Script/Engine.Character|GetCapsuleComponent (Variables|Default|GetParent))) 2.0 5.0 0.0 0.0 "Attack1"))

(fn ConstructionScript
  (|CallParentFunction))