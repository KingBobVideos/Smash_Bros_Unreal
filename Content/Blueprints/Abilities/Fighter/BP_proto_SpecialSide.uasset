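; BP_proto_SpecialSide is a prototype Fighter side special ability that locks the character in place and plays an animation.
; On start it flips on stick input, then after a brief delay stops movement, applies a different gravity setting, disables moving, flipping, jumping and walking off ledges, and plays the animation.
; When the animation ends, it switches the gravity setting and ends the ability, without explicitly re-enabling the other controls.
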(event EventEndAnim
  (params (AnimNo :type Integer))
  (CallFunction|SetGravity "NewEnumerator0" 0.0)
  (CallFunction|EndAbility))

(event EventAbilityStart
  (CallFunction|FliponStick)
  (Utilities|FlowControl|Delay 0.1)
  (CallFunction|StopAllMovement)
  (CallFunction|SetGravity "NewEnumerator1" 0.0)
  (CallFunction|SetMovement false)
  (CallFunction|SetFlip false)
  (CallFunction|SetJump false)
  (CallFunction|PlayAnimation)
  (CallFunction|WalkOffLedge false))

(fn ConstructionScript
  (|CallParentFunction))