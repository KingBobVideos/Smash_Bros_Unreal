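; Prototype up-special ability for a fighter: launches the owning character sharply upward and slightly toward its facing side.
; On start it enables full-body ledge handling, stops movement, allows a brief stick-flip window, then locks flip and jump before playing the animation and launching.
; Tick stops the montage if the character enters a particular state while active.
; When the animation ends, the ability ends and an airborne character enters free fall.
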(event EventTick
  (params (DeltaSeconds :type Float%20%28single-precision%29))
  (|CallParentFunction DeltaSeconds)
  (if (and (Utilities|Enum|Equal(Enum) (Variables|/Game/Blueprints/Characters/BP_Fighter.BP_Fighter_C|GetStates (Variables|Default|GetParent)) "NewEnumerator8") (Variables|Default|GetActive))
    (Animation|StopAnimMontage (Variables|Default|GetParent) (Utilities|Array|Get(acopy) (Variables|Default|GetAnimations)))))

(event EventEndAnim
  (params (AnimNo :type Integer))
  (CallFunction|EndAbility)
  (Utilities|InAir? (Variables|Default|GetParent)
    (:Air
      (CallFunction|FreeFall))))

(event EventAbilityStart
  (bind _parent (Variables|Default|GetParent))
  (CallFunction|FullbodyLedge true)
  (CallFunction|StopAllMovement)
  (CallFunction|FliponStick)
  (Utilities|FlowControl|Delay 0.1)
  (CallFunction|SetFlip false)
  (CallFunction|SetJump false)
  (CallFunction|PlayAnimation)
  (switch Utilities|FlowControl|Switch|SwitchonEnum_faceing (Variables|/Game/Blueprints/Characters/BP_Fighter.BP_Fighter_C|GetFaceing _parent)
    (:NewEnumerator0
      (Default|Launch _parent "0,200.000000,1700.000000" true true))
    (:NewEnumerator1
      (Default|Launch _parent "0,-200.000000,1700.000000" true true))))

(fn ConstructionScript
  (|CallParentFunction))