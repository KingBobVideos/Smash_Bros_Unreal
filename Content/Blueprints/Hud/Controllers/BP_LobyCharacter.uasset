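; Lobby character that represents one player, showing a colored Ready or Not Ready text above a shared lobby state.
; On BeginPlay it takes its player number from BP_lobbyMannager and registers controller, default character and ready flag in the game instance arrays.
; Server and client events update readiness.
; Tick refreshes the text, pushes the player number from authority and reveals the ME marker when the manager's ClientNo matches its nonzero number.
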(event Custom|UpdatePlayerNoClients
  (params (PlayerNo :type Integer))
  ;[1 1 1] PlayerNo
  (Variables|Default|SetPlayerNo PlayerNo))

(event Custom|ReadyUpClients
  (params (Ready :type Boolean) (Index :type Integer))
  ;[0.5734 1 0.5144 1 30] Ready UP
  (bind _output_get (Variables|Default|SetReady Ready))
  (Utilities|Array|SetArrayElem (Variables|/Game/Blueprints/managers/GI_FighterGameInstance.GI_FighterGameInstance_C|GetReadyArray (Variables|Default|GetGameInstance)) Index _output_get true))

(event Custom|ReadyUpServer
  (params (Ready :type Boolean) (Index :type Integer))
  ;[0.5734 1 0.5144 1 30] Ready UP
  (bind _output_get (Variables|Default|SetReady Ready))
  (Utilities|Array|SetArrayElem (Variables|/Game/Blueprints/managers/GI_FighterGameInstance.GI_FighterGameInstance_C|GetReadyArray (Variables|Default|GetGameInstance)) Index _output_get true))

(event Custom|updateNo
  ;[1 1 1] PlayerNo
  (Networking|SwitchHasAuthority
    (:Authority
      (CallFunction|UpdatePlayerNoClients (Variables|Default|GetPlayerNo)))))

(event Custom|SetClient
  (bind _playerno (Variables|Default|GetPlayerNo))
  ;[1 1 1 1 30] SetSelfClent
  (if (and (== (Variables|/Game/Blueprints/managers/BP_lobbyMannager.BP_lobbyMannager_C|GetClientNo (Variables|Default|GetManager)) _playerno) (!= _playerno 0))
    (Rendering|SetVisibility (Variables|Default|GetME) true false)))

(event Custom|ReadyUp
  (params (Index :type Integer))
  ;[0.5734 1 0.5144 1 30] Ready UP
  (CallFunction|ReadyUpServer true Index)
  (CallFunction|ReadyUpClients true Index))

(event Custom|UpdateText
  ;[1 1 1 1 30] ReadyText
  (Rendering|Components|TextRender|SetText (Variables|Default|GetTextRender) (Variables|Default|GetReadyText)))

(event EventBeginPlay
  ;[1 0.7864 0.4562 1 30] Get GM, GI, set player number
  (Utilities|FlowControl|Delay 0.01)
  (bind _asgm_lobby_mode (Utilities|Casting|CastToGM_LobbyMode (Game|GetGameMode))
    (:then
      (Variables|Default|SetlobyMode _asgm_lobby_mode))
    (:CastFailed
      _))
  (bind _asgi_fighter_game_instance (Utilities|Casting|CastToGI_FighterGameInstance (Game|GetGameInstance)))
  (bind _output_get (Variables|Default|SetGameInstance _asgi_fighter_game_instance))
  (bind _outactors (Actor|GetAllActorsOfClass "/Game/Blueprints/managers/BP_lobbyMannager.BP_lobbyMannager_C"))
  (Variables|Default|SetManager (Utilities|Array|Get(acopy) _outactors))
  (Utilities|Array|SetArrayElem (Variables|/Game/Blueprints/managers/GI_FighterGameInstance.GI_FighterGameInstance_C|GetPlayerControllers _output_get) (Variables|/Game/Blueprints/managers/BP_lobbyMannager.BP_lobbyMannager_C|GetNumberOfPlayer (Utilities|Array|Get(acopy) _outactors)) (Pawn|GetController) true)
  (bind _output_get_2 (Variables|Default|SetPlayerNo (Variables|/Game/Blueprints/managers/BP_lobbyMannager.BP_lobbyMannager_C|GetNumberOfPlayer (Utilities|Array|Get(acopy) _outactors))))
  (Utilities|Array|SetArrayElem (Variables|/Game/Blueprints/managers/GI_FighterGameInstance.GI_FighterGameInstance_C|GetPlayerCharacters _output_get) _output_get_2 "NewEnumerator0" true)
  (Utilities|Array|SetArrayElem (Variables|/Game/Blueprints/managers/GI_FighterGameInstance.GI_FighterGameInstance_C|GetReadyArray (Variables|Default|GetGameInstance)) (Variables|Default|GetPlayerNo) false true))

(event EventTick
  (params (DeltaSeconds :type Float%20%28single-precision%29))
  (bind _textrender (Variables|Default|GetTextRender))
  ;[0.4479 0.7066 1 1 30] Set Clients, is clients ready?
  (CallFunction|SetClient)
  (CallFunction|UpdateNo)
  (if (Variables|Default|GetReady)
    (Variables|Default|SetReadyText "Ready")
    (Rendering|Components|TextRender|SetTextRenderColor _textrender (Variables|Default|GetReadyCol))
    (else
      (Variables|Default|SetReadyText "Not Ready")
      (Rendering|Components|TextRender|SetTextRenderColor _textrender (Variables|Default|GetNotReadyCol))))
  (CallFunction|UpdateText))

(fn ConstructionScript)