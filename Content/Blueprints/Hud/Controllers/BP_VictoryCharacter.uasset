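; BP_VictoryCharacter is the player-side Blueprint for the win screen, forwarding Start input to the game mode.
; After a short delay on BeginPlay, it caches GM_winscreen and GI_FighterGameInstance, clears GameLooped, and stores the first PlayerPositions entry as PlayerNo.
; Gamepad Special Right calls PressStartEvent on the game mode.
; Tick only checks FPlayerState validity without acting, and a character lookup is left unconnected.
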(event EventBeginPlay
  ;[1 1 1] Comment
  (Utilities|FlowControl|Delay 0.1)
  (bind _asgm_winscreen (Utilities|Casting|CastToGM_winscreen (Game|GetGameMode)))
  (Variables|Default|SetGameMode _asgm_winscreen)
  (bind _asgi_fighter_game_instance (Utilities|Casting|CastToGI_FighterGameInstance (Game|GetGameInstance)))
  (bind _output_get (Variables|Default|SetGameInstance _asgi_fighter_game_instance))
  (Variables|/Game/Blueprints/managers/GI_FighterGameInstance.GI_FighterGameInstance_C|SetGameLooped _output_get false)
  (Variables|Default|SetPlayerNo (Utilities|Array|Get(acopy) (Variables|/Game/Blueprints/managers/GI_FighterGameInstance.GI_FighterGameInstance_C|GetPlayerPositions _asgi_fighter_game_instance))))

(event EventTick
  (params (DeltaSeconds :type Float%20%28single-precision%29))
  ;[1 1 1] Comment
  (Utilities|IsValid (Variables|Default|GetF_PlayerState)))

(event Input|GamepadEvents|GamepadSpecialRight
  (params (Key :type Key%20Structure))
  ;[1 1 1] Start
  (:Pressed
    (Default|PressStartEvent (Variables|Default|GetGameMode))))

(fn ConstructionScript)