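; Per-player menu controller for the fighter game that relays each local player's input to GM_Menus by controller number.
; Tick turns stick axes into throttled directional events, while select and trigger buttons set per-player flags on the game mode.
; Start or Enter advances by menu state: leaving title, joining character select or starting from map select.
; Once the game mode starts, inactive controllers trigger player removal, with separate handling when CPUs exist.
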(event Custom|StartPressed
  (bind _instance (Variables|Default|Getinstance))
  (bind _gamemode (Variables|Default|GetGameMode))
  (bind _gamemode_2 (Variables|Default|GetGameMode))
  ;[0.1579 0.3698 0.1822 1 30] Start And Enter Input
  (switch Utilities|FlowControl|Switch|SwitchonEnum_menus (Variables|/Game/Blueprints/managers/gamemodes/GM_Menus.GM_Menus_C|GetMenus (Variables|Default|GetGameMode))
    (:NewEnumerator2
      (Utilities|Array|SetArrayElem (Variables|/Game/Blueprints/managers/gamemodes/GM_Menus.GM_Menus_C|GetActiveControllers _gamemode_2) (Variables|Default|GetControllerNo) true true)
      (bind _output_get (Variables|/Game/Blueprints/managers/GI_FighterGameInstance.GI_FighterGameInstance_C|SetActiveControllers _instance (Variables|/Game/Blueprints/managers/gamemodes/GM_Menus.GM_Menus_C|GetActiveControllers _gamemode_2)))
      (Variables|/Game/Blueprints/managers/GI_FighterGameInstance.GI_FighterGameInstance_C|SetNumberOfPlayers _instance (Utilities|Array|Length _output_get))
      (Variables|Default|SetActive true)
      (if (Variables|/Game/Blueprints/managers/gamemodes/GM_Menus.GM_Menus_C|GetAllready _gamemode_2)
        (Variables|/Game/Blueprints/managers/gamemodes/GM_Menus.GM_Menus_C|SetGoToMap _gamemode_2 true)))
    (:NewEnumerator3
      (Default|GameStart (Variables|Default|GetGameMode)))
    (:NewEnumerator8
      (bind _outactors (Actor|GetAllActorsOfClass "/Game/Blueprints/Hud/Menus/Main/HUD_Menus.HUD_Menus_C"))
      (Default|PressStart (Utilities|Array|Get(acopy) _outactors))
      (Variables|/Game/Blueprints/managers/gamemodes/GM_Menus.GM_Menus_C|SetMenus _gamemode "NewEnumerator0")
      (Utilities|Array|SetArrayElem (Variables|/Game/Blueprints/managers/gamemodes/GM_Menus.GM_Menus_C|GetActiveControllers _gamemode) 0 true true)
      (Variables|Default|SetActive true))))

(event Custom|MoveEvent
  (bind _gamemode (Variables|Default|GetGameMode))
  (bind _controllerno (Variables|Default|GetControllerNo))
  ;[1 1 1 1 30] Move Event set to gamemode
  (switch Utilities|FlowControl|Switch|SwitchonEnum_Direction (Variables|Default|GetDirection)
    (:NewEnumerator2
      (Default|UpEvent _gamemode _controllerno))
    (:NewEnumerator3
      (Default|DownEvent _gamemode _controllerno))
    (:NewEnumerator4
      (Default|LeftEvent _gamemode _controllerno))
    (:NewEnumerator5
      (Default|RightEvent _gamemode _controllerno))))

(event EventBeginPlay
  ;[1 1 1 1 30] BeginPlay
  (bind _asgm_menus (Utilities|Casting|CastToGM_Menus (Game|GetGameMode)))
  (Variables|Default|SetGameMode _asgm_menus)
  (bind _asgi_fighter_game_instance (Utilities|Casting|CastToGI_FighterGameInstance (Game|GetGameInstance)))
  (Variables|Default|Setinstance _asgi_fighter_game_instance)
  (for _index (range 0 3)
    (bind _returnvalue (Class|GameplayStatics|GetPlayerControllerID (Game|GetPlayerController _index)))
    (if (== _returnvalue _index)
      (Variables|Default|SetControllerNo _index)
      (Variables|Default|SetActiveControllers (Variables|/Game/Blueprints/managers/gamemodes/GM_Menus.GM_Menus_C|GetActiveControllers (Variables|Default|GetGameMode)))
      (if (Variables|/Game/Blueprints/managers/GI_FighterGameInstance.GI_FighterGameInstance_C|GetGameLooped (Variables|Default|Getinstance))
        (CallFunction|StartPressed)))))

(event EventTick
  (params (DeltaSeconds :type Float%20%28single-precision%29))
  (bind _instance (Variables|Default|Getinstance))
  (bind _updown (Variables|Default|GetUpDown))
  (bind _leftright (Variables|Default|GetLeftRight))
  (bind _cpu (Variables|/Game/Blueprints/managers/GI_FighterGameInstance.GI_FighterGameInstance_C|GetCPU _instance))
  ;[0.9427 0.7002 0.7866 1 30] Tick
  (Utilities|FlowControl|Sequence
    (:then_0
      (if (Variables|Default|GetActive)
        ;[0.2083 0.2083 0.2083 1 30] Directonal inputs
        (Utilities|FlowControl|Sequence
          (:then_0
            (if (<= _updown -0.9)
              (if (Variables|Default|GetCanMove)
                (Variables|Default|SetCanMove false)
                (Variables|Default|SetDirection "NewEnumerator3")
                (CallFunction|MoveEvent)
                (Utilities|FlowControl|Delay 0.2)
                (Variables|Default|SetCanMove true))
              (elif (>= _updown 0.9)
                (if (Variables|Default|GetCanMove)
                  (Variables|Default|SetCanMove false)
                  (Variables|Default|SetDirection "NewEnumerator2")
                  (CallFunction|MoveEvent)
                  (Utilities|FlowControl|Delay 0.2)
                  (Variables|Default|SetCanMove true)))))
          (:then_1
            (if (<= _leftright -0.9)
              (if (Variables|Default|GetCanMove)
                (Variables|Default|SetCanMove false)
                (Variables|Default|SetDirection "NewEnumerator4")
                (CallFunction|MoveEvent)
                (Utilities|FlowControl|Delay 0.2)
                (Variables|Default|SetCanMove true))
              (elif (>= _leftright 0.9)
                (if (Variables|Default|GetCanMove)
                  (Variables|Default|SetCanMove false)
                  (Variables|Default|SetDirection "NewEnumerator5")
                  (CallFunction|MoveEvent)
                  (Utilities|FlowControl|Delay 0.2)
                  (Variables|Default|SetCanMove true))))))))
    (:then_1
      ;[1 0.2083 0.2083 1 30] Remove Unused Players
      (if (and (Variables|/Game/Blueprints/managers/gamemodes/GM_Menus.GM_Menus_C|GetStart (Variables|Default|GetGameMode)) (not (Variables|Default|GetActive)))
        (if (Utilities|Array|ContainsItem _cpu true)
          (for (_array_element _array_index) _cpu
            (if (and (not _array_element) (Utilities|Enum|Equal(Enum) (Utilities|Array|Get(acopy) (Variables|/Game/Blueprints/managers/GI_FighterGameInstance.GI_FighterGameInstance_C|GetPlayerCharacters _instance) _array_index) "NewEnumerator1"))
              (Utilities|Remove _array_index)))
          (else
            (Utilities|Remove (Variables|Default|GetControllerNo))))))))

(event Input|ActionEvents|InputActionMenuSelect
  (params (Key :type Key%20Structure))
  (bind _active (Variables|Default|GetActive))
  (bind _gamemode (Variables|Default|GetGameMode))
  (bind _controllerno (Variables|Default|GetControllerNo))
  (bind _select (Variables|/Game/Blueprints/managers/gamemodes/GM_Menus.GM_Menus_C|GetSelect _gamemode))
  ;[0.066 0.1163 0.2917 1 30] Face Button Input
  (:Pressed
    (if _active
      (Utilities|Array|SetArrayElem _select _controllerno true true)))
  (:Released
    (if _active
      (Utilities|Array|SetArrayElem _select _controllerno false true))))

(event Input|ActionEvents|InputActionMenuBack
  (params (Key :type Key%20Structure))
  (bind _controllerno (Variables|Default|GetControllerNo))
  (bind _gamemode (Variables|Default|GetGameMode))
  (bind _playerselected (Variables|/Game/Blueprints/managers/gamemodes/GM_Menus.GM_Menus_C|GetPlayerSelected _gamemode))
  ;[0.066 0.1163 0.2917 1 30] Face Button Input
  (:Pressed
    (Variables|/Game/Blueprints/managers/gamemodes/GM_Menus.GM_Menus_C|SetBack _gamemode true)
    (if (Utilities|Array|Get(acopy) _playerselected _controllerno)
      (Utilities|Array|SetArrayElem _playerselected _controllerno false)))
  (:Released
    (Variables|/Game/Blueprints/managers/gamemodes/GM_Menus.GM_Menus_C|SetBack _gamemode false)))

(event Input|ActionEvents|InputActionMenuLT
  (params (Key :type Key%20Structure))
  (bind _controllerno (Variables|Default|GetControllerNo))
  (bind _active (Variables|Default|GetActive))
  (bind _gamemode (Variables|Default|GetGameMode))
  (bind _lefttriggers (Variables|/Game/Blueprints/managers/gamemodes/GM_Menus.GM_Menus_C|GetLeftTriggers _gamemode))
  ;[0.2812 0.133 0.2263 1 30] Triggers
  (:Pressed
    (if _active
      (Utilities|Array|SetArrayElem _lefttriggers _controllerno true true)))
  (:Released
    (if _active
      (Utilities|Array|SetArrayElem _lefttriggers _controllerno false true))))

(event Input|ActionEvents|InputActionMenuRT
  (params (Key :type Key%20Structure))
  ;[0.2812 0.133 0.2263 1 30] Triggers
  (:Pressed
    (if (Variables|Default|GetActive)
      (Utilities|Array|SetArrayElem (Variables|/Game/Blueprints/managers/gamemodes/GM_Menus.GM_Menus_C|GetRightTriggers (Variables|Default|GetGameMode)) (Variables|Default|GetControllerNo) true true))))

(event Input|AxisEvents|InputAxisUpDown
  (params (AxisValue :type Float%20%28single-precision%29))
  ;[1 1 1 1 30] Directon Input
  (Variables|Default|SetUpDown AxisValue))

(event Input|AxisEvents|InputAxisLeftRight
  (params (AxisValue :type Float%20%28single-precision%29))
  ;[1 1 1 1 30] Directon Input
  (Variables|Default|SetLeftRight AxisValue))

(event Input|KeyboardEvents|Enter
  (params (Key :type Key%20Structure))
  ;[0.1579 0.3698 0.1822 1 30] Start And Enter Input
  (:Pressed
    (CallFunction|StartPressed)))

(event Input|GamepadEvents|GamepadSpecialRight
  (params (Key :type Key%20Structure))
  ;[0.1579 0.3698 0.1822 1 30] Start And Enter Input
  (:Pressed
    (CallFunction|StartPressed)))

(fn ConstructionScript)