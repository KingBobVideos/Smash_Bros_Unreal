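; Grabbable stage ledge for BP_Fighter characters, facing Left or Right.
; The construction script shows the trigger box for that Direction and offsets HandLocation to that side.
; On overlap by the fighter's ledge detector, or body if FullBodyLedgeGrab, it turns the fighter, passes HandLocation and calls LedgeGrab unless on cooldown or already hanging.
; LedgeHog makes an occupied ledge block grabs; Tick frees it once the stored fighter leaves the ledge state.
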(event OnComponentBeginOverlap(leftBox)
  (params (OverlappedComponent :type Primitive%20Component%20Object%20Reference) (OtherActor :type Actor%20Object%20Reference) (OtherComp :type Primitive%20Component%20Object%20Reference) (OtherBodyIndex :type Integer) (bFromSweep :type Boolean) (SweepResult :type Hit%20Result%20Structure%20%28by%20ref%29))
  ;[1 1 1] Comment
  (if (not (and (Variables|Default|GetOcubied) (Variables|Default|GetLedgeHog)))
    (bind _asbp_fighter (Utilities|Casting|CastToBP_Fighter OtherActor))
    (bind _output_get (Variables|Default|Setfighter _asbp_fighter))
    (if (or (and (Variables|/Game/Blueprints/Characters/BP_Fighter.BP_Fighter_C|GetFullBodyLedgeGrab _asbp_fighter) (== _output_get OtherActor)) (== OtherComp (Variables|/Game/Blueprints/Characters/BP_Fighter.BP_Fighter_C|GetLedgeDectector _output_get)))
      (switch Utilities|FlowControl|Switch|SwitchonEnum_faceing (Variables|Default|Getdirection)
        (:NewEnumerator0
          (Variables|/Game/Blueprints/Characters/BP_Fighter.BP_Fighter_C|SetFaceing (Variables|Default|Getfighter) "NewEnumerator1")
          (Transformation|SetWorldRotation (Variables|/Script/Engine.Character|GetCapsuleComponent (Variables|Default|Getfighter)) "0.000000,-90.000000,0.000000" false false)
          (Variables|/Game/Blueprints/Characters/BP_Fighter.BP_Fighter_C|SetLedgeLocation (Variables|Default|Getfighter) (Variables|Default|GetHandLocation))
          (if (and (Utilities|Enum|NotEqual(Enum) (Variables|/Game/Blueprints/Characters/BP_Fighter.BP_Fighter_C|GetStates (Variables|Default|Getfighter)) "NewEnumerator8") (not (Variables|/Game/Blueprints/Characters/BP_Fighter.BP_Fighter_C|GetLedgeCooldown (Variables|Default|Getfighter))))
            (Default|LedgeGrab (Variables|Default|Getfighter))
            (Variables|Default|SetOcubied true)))))))

(event OnComponentBeginOverlap(rightBox)
  (params (OverlappedComponent :type Primitive%20Component%20Object%20Reference) (OtherActor :type Actor%20Object%20Reference) (OtherComp :type Primitive%20Component%20Object%20Reference) (OtherBodyIndex :type Integer) (bFromSweep :type Boolean) (SweepResult :type Hit%20Result%20Structure%20%28by%20ref%29))
  ;[1 1 1] Comment
  (if (not (and (Variables|Default|GetOcubied) (Variables|Default|GetLedgeHog)))
    (bind _asbp_fighter (Utilities|Casting|CastToBP_Fighter OtherActor))
    (bind _output_get (Variables|Default|Setfighter _asbp_fighter))
    (if (or (== OtherComp (Variables|/Game/Blueprints/Characters/BP_Fighter.BP_Fighter_C|GetLedgeDectector _asbp_fighter)) (and (Variables|/Game/Blueprints/Characters/BP_Fighter.BP_Fighter_C|GetFullBodyLedgeGrab _asbp_fighter) (== _output_get OtherActor)))
      (switch Utilities|FlowControl|Switch|SwitchonEnum_faceing (Variables|Default|Getdirection)
        (:NewEnumerator1
          (Variables|/Game/Blueprints/Characters/BP_Fighter.BP_Fighter_C|SetFaceing (Variables|Default|Getfighter) "NewEnumerator0")
          (Transformation|SetWorldRotation (Variables|/Script/Engine.Character|GetCapsuleComponent (Variables|Default|Getfighter)) "0.000000,90.000000,0.000000" false false)
          (Variables|/Game/Blueprints/Characters/BP_Fighter.BP_Fighter_C|SetLedgeLocation (Variables|Default|Getfighter) (Variables|Default|GetHandLocation))
          (if (and (Utilities|Enum|NotEqual(Enum) (Variables|/Game/Blueprints/Characters/BP_Fighter.BP_Fighter_C|GetStates (Variables|Default|Getfighter)) "NewEnumerator8") (not (Variables|/Game/Blueprints/Characters/BP_Fighter.BP_Fighter_C|GetLedgeCooldown (Variables|Default|Getfighter))))
            (Default|LedgeGrab (Variables|Default|Getfighter))
            (Variables|Default|SetOcubied true)))))))

(event EventTick
  (params (DeltaSeconds :type Float%20%28single-precision%29))
  ;[1 1 1] Comment
  (Utilities|IsValid (Variables|Default|Getfighter)
    (:Is%20Valid
      (if (Utilities|Enum|NotEqual(Enum) (Variables|/Game/Blueprints/Characters/BP_Fighter.BP_Fighter_C|GetStates (Variables|Default|Getfighter)) "NewEnumerator8")
        (Variables|Default|SetOcubied false)
        (Variables|Default|Setfighter 0)))))

(fn ConstructionScript
  (bind _defaultsceneroot (Variables|Default|GetDefaultSceneRoot))
  (bind _returnvalue (Transformation|GetWorldLocation _defaultsceneroot))
  (switch Utilities|FlowControl|Switch|SwitchonEnum_faceing (Variables|Default|Getdirection)
    (:NewEnumerator0
      (Rendering|SetVisibility (Variables|Default|GetleftBox) true false)
      (Rendering|SetVisibility (Variables|Default|GetrightBox) false false)
      (Variables|Default|SetHandLocation (+ _returnvalue "0,50.000000, 0")))
    (:NewEnumerator1
      (Rendering|SetVisibility (Variables|Default|GetleftBox) false false)
      (Rendering|SetVisibility (Variables|Default|GetrightBox) true false)
      (Variables|Default|SetHandLocation (+ _returnvalue "0,-50.000000, 0")))))