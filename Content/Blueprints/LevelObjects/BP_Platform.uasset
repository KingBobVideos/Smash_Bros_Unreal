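; BP_Platform is a one-way platform that BP_Fighter characters stand on from above and pass through from below.
; On BeginPlay, its Number picks one of five custom collision channels for the Cube, printing a warning for some invalid values.
; Every Tick, it sets each fighter's capsule to block that channel only while the feet are above the platform's Z and PlatPhaze is off, otherwise to ignore it.
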(event EventBeginPlay
  (bind _cube (Variables|Default|GetCube))
  ;[1 1 1 1 25] Set Collision Channle
  (switch int (Variables|Default|GetNumber)
    (:Default
      (Development|PrintString "SET PLATFORM NUMBER!" true true "(R=1.000000,G=0.000000,B=0.130888,A=1.000000)"))
    (:0
      (Collision|SetCollisionObjectType _cube "ECC_GameTraceChannel1")
      (Variables|Default|SetPlats "ECC_GameTraceChannel1"))
    (:1
      (Collision|SetCollisionObjectType _cube "ECC_GameTraceChannel2")
      (Variables|Default|SetPlats "ECC_GameTraceChannel2"))
    (:2
      (Collision|SetCollisionObjectType _cube "ECC_GameTraceChannel3")
      (Variables|Default|SetPlats "ECC_GameTraceChannel3"))
    (:3
      (Collision|SetCollisionObjectType _cube "ECC_GameTraceChannel4")
      (Variables|Default|SetPlats "ECC_GameTraceChannel4"))
    (:4
      (Collision|SetCollisionObjectType _cube "ECC_GameTraceChannel5")
      (Variables|Default|SetPlats "ECC_GameTraceChannel5"))
    (:5
      (Development|PrintString "EXCEEDED VALUE RANGE FOR PLATFORMS! ADD NEW COLLISION CHANNELS " true true "(R=1.000000,G=0.000000,B=0.130888,A=1.000000)"))))

(event EventTick
  (params (DeltaSeconds :type Float%20%28single-precision%29))
  (bind _plats (Variables|Default|GetPlats))
  ;[1 1 1 1 25] Comment
  (Variables|Default|SetZpos (.Z (Math|Vector|BreakVector (Transformation|GetActorLocation))))
  (bind _outactors (Actor|GetAllActorsOfClass "/Game/Blueprints/Characters/BP_Fighter.BP_Fighter_C"))
  (for _array_element _outactors
    (if (> (Variables|/Game/Blueprints/Characters/BP_Fighter.BP_Fighter_C|GetFootZPos _array_element) (Variables|Default|GetZpos))
      (if (not (Variables|/Game/Blueprints/Characters/BP_Fighter.BP_Fighter_C|GetPlatPhaze _array_element))
        (Collision|SetCollisionResponsetoChannel (Variables|/Script/Engine.Character|GetCapsuleComponent _array_element) _plats "ECR_Block")
        (else
          (Collision|SetCollisionResponsetoChannel (Variables|/Script/Engine.Character|GetCapsuleComponent _array_element) _plats "ECR_Ignore" :!label _label)))
      (else
        (goto _label)))))

(fn ConstructionScript)