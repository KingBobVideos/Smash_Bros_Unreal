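; Shared platform-fighter camera that becomes the player's view and follows all fighters flagged for tracking until the game ends.
; Each tick it re-gathers fighters and eases toward their average Y/Z position plus a height offset, using a swept move.
; Zoom is a depth offset on X from the larger clamped Y or Z spread, smoothed only when horizontal.
; It finds a camera volume, but its bounds clamp is unused.
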(event Custom|UpdateCamera
  ;[1 0.5714 0.7567 1 25] Update Camera
  (Game|Player|SetViewTargetwithBlend (Game|GetPlayerController 0) self 0.0 "VTBlend_Linear" 0.0 false))

(event EventBeginPlay
  ;[1 0.8394 0.5265 1 25] start
  (Utilities|FlowControl|Delay 1.0)
  (bind _asgi_fighter_game_instance (Utilities|Casting|CastToGI_FighterGameInstance (Game|GetGameInstance)))
  (Variables|Default|SetInstance _asgi_fighter_game_instance)
  (bind _asgm_plat_fighter_gamemode (Utilities|Casting|CastToGM_PlatFighterGamemode (Game|GetGameMode))
    (:then
      (Variables|Default|SetGameMode _asgm_plat_fighter_gamemode))
    (:CastFailed
      _))
  (bind _outactors (Actor|GetAllActorsOfClass "/Game/Blueprints/Characters/BP_Fighter.BP_Fighter_C"))
  (Variables|Default|Setfighters _outactors)
  (Game|Player|SetViewTargetwithBlend (Game|GetPlayerController 0) self 0.0 "VTBlend_Linear" 0.0 false)
  (Utilities|FlowControl|Delay 0.1)
  (Variables|Default|SetTracking true)
  (Variables|Default|SetXpos (.X (Math|Vector|BreakVector (Transformation|GetWorldLocation (Variables|Default|GetCamera)))))
  (bind _outactors_2 (Actor|GetAllActorsOfClass "/Game/Blueprints/LevelObjects/BP_CameraVolume.BP_CameraVolume_C"))
  (for (_array_element _array_index) _outactors_2
    (if (== _array_index 0)
      (Variables|Default|SetCambounds _array_element))))

(event EventTick
  (params (DeltaSeconds :type Float%20%28single-precision%29))
  ;[0.2424 0.2604 0.2197 1 25] Tick, is tracking
  (Variables|Default|SetDelta DeltaSeconds)
  (if (Variables|Default|GetTracking)
    (bind _outactors (Actor|GetAllActorsOfClass "/Game/Blueprints/Characters/BP_Fighter.BP_Fighter_C"))
    (Variables|Default|Setfighters _outactors)
    (Utilities|FlowControl|Sequence
      (:then_0
        ;;[0.3794 0.599 0.2839 1 25] Tracking
        (CallFunction|TrackingFunc (Variables|Default|GetDelta))
        (CallFunction|UpdateCamera)
        (CallFunction|GetDistanceBetweenFighters))
      (:then_1
        ;;[0.5979 0.7549 1] Stop Tracking on end
        (if (Variables|/Game/Blueprints/managers/GI_FighterGameInstance.GI_FighterGameInstance_C|GetEndGame (Variables|Default|GetInstance))
          (Variables|Default|SetTracking false)))
      (:then_2
        ;;[0.4892 1 0.8273] Zoom Clamp
        (if (> (Variables|Default|GetZoom) (Variables|Default|GetZoomMax))
          (Variables|Default|SetZoom (Variables|Default|GetZoomMax)))))))

(fn ConstructionScript)

(fn GetDistanceBetweenFighters
  (bind _zarray (Variables|Default|GetZArray))
  (bind _yarray (Variables|Default|GetYArray))
  (for (_array_element _array_index) (Variables|Default|Getfighters)
    (if (Variables|/Game/Blueprints/Characters/BP_Fighter.BP_Fighter_C|GetTrackCam _array_element)
      ;[0.9363 0.5879 1 1 25] Get The Y and Z positions and add to array
      (Utilities|Array|SetArrayElem (Variables|Default|GetYArray) _array_index (.Y (Math|Vector|BreakVector (Transformation|GetWorldLocation (Variables|/Script/Engine.Character|GetCapsuleComponent _array_element)))) true)
      (Utilities|Array|SetArrayElem (Variables|Default|GetZArray) _array_index (.Z (Math|Vector|BreakVector (Transformation|GetWorldLocation (Variables|/Script/Engine.Character|GetCapsuleComponent _array_element)))) true)
      (else
        ;[0.6667 0.4134 0.3465 1 25] Set Y and Z to 0 when not tracking
        (Utilities|Array|SetArrayElem (Variables|Default|GetYArray) _array_index 0.0 true)
        (Utilities|Array|SetArrayElem (Variables|Default|GetZArray) _array_index 0.0 true)))
    ;[0.4133 0.9402 1 1 25] Set cam zoom
    (bind _output_get (Variables|Default|SetZLow (.MaxValue (Math|Float|MaxOfFloatArray _zarray))))
    (bind _output_get_2 (Variables|Default|SetZTop (.MinValue (Math|Float|MinOfFloatArray _zarray))))
    (bind _output_get_3 (Variables|Default|SetYLeft (.MaxValue (Math|Float|MaxOfFloatArray _yarray))))
    (bind _output_get_4 (Variables|Default|SetYRight (.MinValue (Math|Float|MinOfFloatArray _yarray))))
    (if (> (- _output_get _output_get_2) (- _output_get_3 _output_get_4))
      (bind _output_get_5 (Variables|Default|SetZoom (Math|Float|Clamp(Float) (- _output_get _output_get_2) (Variables|Default|GetZoomMin) (Variables|Default|GetZoomMax))))
      (else
        (Variables|Default|SetZoom (Math|Interpolation|FInterpTo (Variables|Default|GetZoom) (- (Math|Float|Clamp(Float) (- _output_get_3 _output_get_4) (Variables|Default|GetZoomMin) (Variables|Default|GetZoomMax)) (/ (Math|Float|Clamp(Float) (- _output_get_3 _output_get_4) (Variables|Default|GetZoomMin) (Variables|Default|GetZoomMax)) 4.0)) (Variables|Default|GetDelta) 3.0))))))

(fn TrackingFunc
  (params (DeltaTime :type Float%20%28single-precision%29))
  (bind _trackedfighters (Variables|Default|GetTrackedFighters))
  (bind _camera (Variables|Default|GetCamera))
  (for (_array_element _array_index) (Variables|Default|Getfighters)
    (if (Variables|/Game/Blueprints/Characters/BP_Fighter.BP_Fighter_C|GetTrackCam _array_element)
      (Utilities|Array|SetArrayElem _trackedfighters _array_index _array_element true)
      (else
        (Utilities|Array|SetArrayElem _trackedfighters _array_index 0 true))))
  (bind _returnvalue (Class|GameplayStatics|GetActorArrayAverageLocation (Variables|Default|GetTrackedFighters)))
  (Transformation|SetWorldLocation _camera (Math|Interpolation|VInterpTo (Transformation|GetWorldLocation _camera) (Math|Vector|MakeVector (+ (Variables|Default|GetXpos) (Variables|Default|GetZoom)) (.Y (Math|Vector|BreakVector _returnvalue)) (+ (.Z (Math|Vector|BreakVector _returnvalue)) (Variables|Default|GetCamZOffest))) DeltaTime 4.0) true false))