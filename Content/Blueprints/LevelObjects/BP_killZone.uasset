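; BP_killZone is a level object that kills any BP_Fighter entering its Box by calling KillPlayer.
; With KillOnlyInHitStates on, it spares fighters in one specific state, as the nested check for two other states can never pass there.
; Fighters in every other state die regardless of that flag.
; It also caches all fighters shortly after BeginPlay, but the overlap logic never uses that list.
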(event OnComponentBeginOverlap(Box)
  (params (OverlappedComponent :type Primitive%20Component%20Object%20Reference) (OtherActor :type Actor%20Object%20Reference) (OtherComp :type Primitive%20Component%20Object%20Reference) (OtherBodyIndex :type Integer) (bFromSweep :type Boolean) (SweepResult :type Hit%20Result%20Structure%20%28by%20ref%29))
  ;[0.7299 1 0.5594] Kill Fighter on overlap
  (bind _asbp_fighter (Utilities|Casting|CastToBP_Fighter OtherActor))
  (if (and (Variables|Default|GetKillOnlyInHitStates) (Utilities|Enum|Equal(Enum) (Variables|/Game/Blueprints/Characters/BP_Fighter.BP_Fighter_C|GetStates _asbp_fighter) "NewEnumerator9"))
    (if (and (or (Utilities|Enum|Equal(Enum) (Variables|/Game/Blueprints/Characters/BP_Fighter.BP_Fighter_C|GetStates _asbp_fighter) "NewEnumerator5") (Utilities|Enum|Equal(Enum) (Variables|/Game/Blueprints/Characters/BP_Fighter.BP_Fighter_C|GetStates _asbp_fighter) "NewEnumerator6")) (Utilities|Enum|NotEqual(Enum) (Variables|/Game/Blueprints/Characters/BP_Fighter.BP_Fighter_C|GetStates _asbp_fighter) "NewEnumerator9"))
      (Default|KillPlayer _asbp_fighter :!label _label))
    (else
      (goto _label))))

(event EventBeginPlay
  ;[1 0.5926 0.4618] Get Fighters
  (Utilities|FlowControl|Delay 0.2)
  (bind _outactors (Actor|GetAllActorsOfClass "/Game/Blueprints/Characters/BP_Fighter.BP_Fighter_C"))
  (Variables|Default|SetFighters _outactors))

(fn ConstructionScript)