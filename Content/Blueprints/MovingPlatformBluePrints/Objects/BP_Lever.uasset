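; Interactable lever that activates a linked spline platform and sets its travel direction.
; A box overlap shows a text prompt; Tick polls Target's Interact flag to flip On/Off, with a short debounce delay.
; Each state maps to a configurable forward or backward direction, pushed to the platform every tick alongside the lever's pitch.
; The character cast is unfinished: overlap clears Target to None.
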(event OnComponentBeginOverlap(Box)
  (params (OverlappedComponent :type Primitive%20Component%20Object%20Reference) (OtherActor :type Actor%20Object%20Reference) (OtherComp :type Primitive%20Component%20Object%20Reference) (OtherBodyIndex :type Integer) (bFromSweep :type Boolean) (SweepResult :type Hit%20Result%20Structure%20%28by%20ref%29))
  ;[1 0 0.06137] SetToOwnCharacter
  (bind _asbp_third_person_character (Utilities|Casting|CastTo OtherActor))
  (Variables|Default|SetTarget 0 _asbp_third_person_character)
  (Variables|Default|SetOverlaping true)
  (Rendering|SetVisibility (Variables|Default|GetTextRender) true false))

(event OnComponentEndOverlap(Box)
  (params (OverlappedComponent :type Primitive%20Component%20Object%20Reference) (OtherActor :type Actor%20Object%20Reference) (OtherComp :type Primitive%20Component%20Object%20Reference) (OtherBodyIndex :type Integer))
  ;[1 0 0.06137] SetToOwnCharacter
  (Utilities|Casting|CastTo OtherActor)
  (Variables|Default|SetOverlaping false)
  (Rendering|SetVisibility (Variables|Default|GetTextRender) false false))

(event Custom|LeverChange
  (params (DeltaTime :type Float%20%28single-precision%29))
  (switch Utilities|FlowControl|Switch|SwitchonEnum_OnOff (Variables|Default|GetOnOff)
    (:NewEnumerator0
      (Transformation|SetRelativeRotation (Variables|Default|GetSM_lever) (Math|Rotator|MakeRotator 0.0 (Math|Interpolation|FInterpTo (Variables|Default|GetOffRotation) (Variables|Default|GetOnRotation) DeltaTime 0.1) 0.0) false false))
    (:NewEnumerator1
      (Transformation|SetRelativeRotation (Variables|Default|GetSM_lever) (Math|Rotator|MakeRotator 0.0 (Math|Interpolation|FInterpTo (Variables|Default|GetOnRotation) (Variables|Default|GetOffRotation) DeltaTime 0.1) 0.0) false false))))

(event EventTick
  (params (DeltaSeconds :type Float%20%28single-precision%29))
  (bind _target (Variables|Default|GetTarget))
  (CallFunction|LeverChange DeltaSeconds)
  (CallFunction|OnOffFunctions)
  (Utilities|IsValid _target
    (:Is%20Valid
      (Variables|Default|SetInteract (Variables|Default|GetInteract _target))
      (if (Math|Boolean|ANDBoolean (Variables|Default|GetInteract) (Variables|Default|GetOverlaping) (not (Variables|Default|GetInteracted)))
        (Variables|Default|SetInteracted true)
        (switch Utilities|FlowControl|Switch|SwitchonEnum_OnOff (Variables|Default|GetOnOff)
          (:NewEnumerator0
            (Variables|Default|SetOnOff "NewEnumerator1"))
          (:NewEnumerator1
            (Variables|Default|SetOnOff "NewEnumerator0")))
        (Variables|/Game/Blueprints/MovingPlatformBluePrints/Platforms/BP_SplinePlatform.BP_SplinePlatform_C|SetActivated (Variables|Default|GetsplinePlat) true)
        (Utilities|FlowControl|Delay 0.2)
        (Variables|Default|SetInteracted false)))))

(fn ConstructionScript
  (Rendering|SetVisibility (Variables|Default|GetTextRender) false false)
  (Transformation|AttachComponentToComponent (Variables|Default|GetSM_lever) (Variables|Default|GetCube) "hing" "KeepRelative" "KeepRelative" "KeepRelative" true)
  (switch Utilities|FlowControl|Switch|SwitchonEnum_OnOff (Variables|Default|GetOnOff)
    (:NewEnumerator0
      (Transformation|SetRelativeRotation (Variables|Default|GetSM_lever) (Math|Rotator|MakeRotator 0.0 (Variables|Default|GetOnRotation) 0.0) false false))
    (:NewEnumerator1
      (Transformation|SetRelativeRotation (Variables|Default|GetSM_lever) (Math|Rotator|MakeRotator 0.0 (Variables|Default|GetOffRotation) 0.0) false false))))

(fn OnOffFunctions
  (bind _splineplat (Variables|Default|GetsplinePlat))
  (switch Utilities|FlowControl|Switch|SwitchonEnum_OnOff (Variables|Default|GetOnOff)
    (:NewEnumerator0
      (switch Utilities|FlowControl|Switch|SwitchonEnum_OnOffFunctions (Variables|Function|GetOnFunction)
        (:NewEnumerator1
          (Variables|/Game/Blueprints/MovingPlatformBluePrints/Platforms/BP_SplinePlatform.BP_SplinePlatform_C|SetBackForward _splineplat "NewEnumerator0"))
        (:NewEnumerator5
          (Variables|/Game/Blueprints/MovingPlatformBluePrints/Platforms/BP_SplinePlatform.BP_SplinePlatform_C|SetBackForward _splineplat "NewEnumerator1"))))
    (:NewEnumerator1
      (switch Utilities|FlowControl|Switch|SwitchonEnum_OnOffFunctions (Variables|Function|GetOffFunction)
        (:NewEnumerator1
          (Variables|/Game/Blueprints/MovingPlatformBluePrints/Platforms/BP_SplinePlatform.BP_SplinePlatform_C|SetBackForward _splineplat "NewEnumerator0"))
        (:NewEnumerator5
          (Variables|/Game/Blueprints/MovingPlatformBluePrints/Platforms/BP_SplinePlatform.BP_SplinePlatform_C|SetBackForward _splineplat "NewEnumerator1"))))))