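; BP_PlatformTriggerZone is a trigger volume that detects when a specific moving platform enters its box.
; Box overlaps are cast to BP_SplinePlatform or BP_Platform and compared against the SplinePlatform or Platform reference.
; A match passes through a DoOnce and sets the Triggerd flag.
; With TriggerOnce the flag stays set; otherwise it pulses briefly, then clears and resets the DoOnce for another trigger.
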(event OnComponentBeginOverlap(Box)
  (params (OverlappedComponent :type Primitive%20Component%20Object%20Reference) (OtherActor :type Actor%20Object%20Reference) (OtherComp :type Primitive%20Component%20Object%20Reference) (OtherBodyIndex :type Integer) (bFromSweep :type Boolean) (SweepResult :type Hit%20Result%20Structure%20%28by%20ref%29))
  (Utilities|FlowControl|Sequence
    (:then_0
      (bind _asbp_spline_platform (Utilities|Casting|CastToBP_SplinePlatform OtherActor)))
    (:then_1
      (bind _asbp_platform (Utilities|Casting|CastToBP_Platform OtherActor))))
  (if (and (or (== _asbp_spline_platform (Variables|Default|GetSplinePlatform)) (== _asbp_platform (Variables|Default|GetPlatform))) (not (Variables|Default|GetTriggerd)))
    (Utilities|FlowControl|DoOnce false
      (:Completed
        (if (Variables|Default|GetTriggerOnce)
          (Variables|Default|SetTriggerd true)
          (else
            (Variables|Default|SetTriggerd true)
            (Utilities|FlowControl|Delay 0.1)
            (Variables|Default|SetTriggerd false)
            (CallFunction|Reset)))))))

(event Custom|Reset
  (Utilities|FlowControl|DoOnce false) ; enters at Reset
)

(fn ConstructionScript)