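; BP_button is a trigger button that activates linked spline moving platforms, calling InVolume when pressed and ExitVolume when released.
; Its box responds to either BP_Fighter or activator items, depending on ItemsActivated.
; Overlap swaps the mesh and triggers platforms directly, or with PressInteract shows a text prompt while Tick polls Interact to toggle them.
; Each change plays a sound, with collision disabled during interact toggles and restored after a short delay.
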(event OnComponentBeginOverlap(Box)
  (params (OverlappedComponent :type Primitive%20Component%20Object%20Reference) (OtherActor :type Actor%20Object%20Reference) (OtherComp :type Primitive%20Component%20Object%20Reference) (OtherBodyIndex :type Integer) (bFromSweep :type Boolean) (SweepResult :type Hit%20Result%20Structure%20%28by%20ref%29))
  ;[0.4993 1 0.4736 1 30] OverlapVolume
  (Variables|Default|SetOverlaping true)
  (if (Variables|Default|GetItemsActivated)
    (bind _asbp_acitivator_item (Utilities|Casting|CastToBP_acitivatorItem OtherActor))
    (Utilities|IsValid _asbp_acitivator_item
      (:Is%20Valid
        _))
    (else
      (bind _asbp_fighter (Utilities|Casting|CastToBP_Fighter OtherActor))
      (Variables|Default|SetTarget _asbp_fighter)))
  (CallFunction|Overlap))

(event OnComponentEndOverlap(Box)
  (params (OverlappedComponent :type Primitive%20Component%20Object%20Reference) (OtherActor :type Actor%20Object%20Reference) (OtherComp :type Primitive%20Component%20Object%20Reference) (OtherBodyIndex :type Integer))
  ;[1 0.5379 0.3147 1 30] ExitVolume
  (Variables|Default|SetOverlaping false)
  (if (Variables|Default|GetItemsActivated)
    (bind _asbp_acitivator_item (Utilities|Casting|CastToBP_acitivatorItem OtherActor))
    (Utilities|IsValid _asbp_acitivator_item
      (:Is%20Valid
        _))
    (else
      (Utilities|Casting|CastToBP_Fighter OtherActor)))
  (CallFunction|EndOverlap))

(event Custom|Overlap
  ;[0.4993 1 0.4736 1 30] OverlapVolume
  (if (Variables|Default|GetPressInteract)
    (Rendering|SetVisibility (Variables|Default|GetTextRender) true false)
    (else
      (Components|StaticMesh|SetStaticMesh (Variables|Default|GetCube) (Variables|Default|GetPressedMesh))
      (CallFunction|EnterVol))))

(event Custom|EnterVol
  (bind _self self)
  (for _array_element (Variables|Platfroms|GetLinkedPlatformsSpline)
    (Default|InVolume _array_element))
  (Audio|PlaySoundatLocation _self (Variables|Default|GetActiveateSound) (Transformation|GetWorldLocation (Variables|Default|GetCube _self)) "0, 0, 0" 1.0 1.0 0.0 0 0 0)
  (Utilities|FlowControl|Delay 0.5)
  (Collision|SetCollisionEnabled (Variables|Default|GetBox) "QueryAndPhysics"))

(event Custom|EndOverlap
  ;[1 0.5379 0.3147 1 30] ExitVolume
  (if (Variables|Default|GetPressInteract)
    (Rendering|SetVisibility (Variables|Default|GetTextRender) false false)
    (else
      (Components|StaticMesh|SetStaticMesh (Variables|Default|GetCube) (Variables|Default|GetUnpressedMesh))
      (CallFunction|ExitVol))))

(event Custom|ExitVol
  (bind _self self)
  (for _array_element (Variables|Platfroms|GetLinkedPlatformsSpline)
    (Default|ExitVolume _array_element))
  (Audio|PlaySoundatLocation _self (Variables|Default|GetActiveateSound) (Transformation|GetWorldLocation (Variables|Default|GetCube _self)) "0, 0, 0" 1.0 1.0 0.0 0 0 0)
  (Utilities|FlowControl|Delay 0.5)
  (Collision|SetCollisionEnabled (Variables|Default|GetBox) "QueryAndPhysics"))

(event EventBeginPlay
  (Rendering|SetVisibility (Variables|Default|GetTextRender) false false))

(event EventTick
  (params (DeltaSeconds :type Float%20%28single-precision%29))
  ;[1 1 1 1 30] Comment
  (Utilities|IsValid (Variables|Default|GetTarget)
    (:Is%20Valid
      (if (Math|Boolean|ANDBoolean (Variables|Default|GetPressInteract) (Variables|Default|GetInteract) (Variables|Default|GetOverlaping) (not (Variables|Default|GetInteracted)))
        (Variables|Default|SetInteracted true)
        (Collision|SetCollisionEnabled (Variables|Default|GetBox) "NoCollision")
        (CallFunction|EnterVol)
        (elif (Math|Boolean|ANDBoolean (Variables|Default|GetPressInteract) (Variables|Default|GetInteract) (Variables|Default|GetOverlaping) (Variables|Default|GetInteracted))
          (Variables|Default|SetInteracted false)
          (Collision|SetCollisionEnabled (Variables|Default|GetBox) "NoCollision")
          (CallFunction|ExitVol))))))

(fn ConstructionScript
  (Components|StaticMesh|SetStaticMesh (Variables|Default|GetCube) (Variables|Default|GetUnpressedMesh))
  (if (Variables|Default|GetPressInteract)
    (Rendering|SetVisibility (Variables|Default|GetTextRender) true false)
    (else
      (Rendering|SetVisibility (Variables|Default|GetTextRender) false false))))