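; Spline-following platform for BP_Fighter levels that can also act as a triggered door or damage zone.
; Each tick it steps a distance along the spline, with optional rotation, end waits, teleport-to-start and stopping.
; Its number picks a collision channel, which each fighter blocks only with feet above it and not phasing, making it one-way.
; The trigger box can activate movement, reverse the door on exit and hit the fighter once per entry.
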(event OnComponentBeginOverlap(Box)
  (params (OverlappedComponent :type Primitive%20Component%20Object%20Reference) (OtherActor :type Actor%20Object%20Reference) (OtherComp :type Primitive%20Component%20Object%20Reference) (OtherBodyIndex :type Integer) (bFromSweep :type Boolean) (SweepResult :type Hit%20Result%20Structure%20%28by%20ref%29))
  ;[1 0.9644 0.376 1 30] Overlap Trigger Box
  (bind _asbp_fighter (Utilities|Casting|CastToBP_Fighter OtherActor))
  (Variables|Default|SetCharacter _asbp_fighter)
  (if (Variables|Main|GetUseVolume)
    (CallFunction|InVolume)))

(event OnComponentEndOverlap(Box)
  (params (OverlappedComponent :type Primitive%20Component%20Object%20Reference) (OtherActor :type Actor%20Object%20Reference) (OtherComp :type Primitive%20Component%20Object%20Reference) (OtherBodyIndex :type Integer))
  ;[1 0.9644 0.376 1 30] Overlap Trigger Box
  (Utilities|Casting|CastToBP_Fighter OtherActor)
  (if (Variables|Main|GetUseVolume)
    (CallFunction|ExitVolume)))

(event Custom|ExitVolume
  ;[1 1 1 1 30] Door Exit Volume
  (Utilities|FlowControl|Sequence
    (:then_0
      (Utilities|ApplyDamage?) ; enters at Reset
    )
    (:then_1
      (if (Variables|Main|GetFunctionAsDoor)
        (Variables|Default|SetBackForward "NewEnumerator1")
        (Variables|Default|SetactiveState "NewEnumerator0")
        (else
          (Variables|Default|SetActivated false))))))

(event Custom|Phase
  (bind _plats (Variables|Default|GetPlats))
  ;[1 1 1 1 25] Comment
  (Variables|Default|SetZpos (.Z (Math|Vector|BreakVector (Transformation|GetWorldLocation (Variables|Components|GetPlatform)))))
  (bind _outactors (Actor|GetAllActorsOfClass "/Game/Blueprints/Characters/BP_Fighter.BP_Fighter_C"))
  (for _array_element _outactors
    (if (> (Variables|/Game/Blueprints/Characters/BP_Fighter.BP_Fighter_C|GetFootZPos _array_element) (Variables|Default|GetZpos))
      (if (not (Variables|/Game/Blueprints/Characters/BP_Fighter.BP_Fighter_C|GetPlatPhaze _array_element))
        (Collision|SetCollisionResponsetoChannel (Variables|/Script/Engine.Character|GetCapsuleComponent _array_element) _plats "ECR_Block")
        (else
          (Collision|SetCollisionResponsetoChannel (Variables|/Script/Engine.Character|GetCapsuleComponent _array_element) _plats "ECR_Ignore" :!label _label)))
      (else
        (goto _label)))))

(event Custom|InVolume
  (Variables|Default|SetActivated true)
  (Utilities|ApplyDamage?
    (:output
      ;[1 1 1 1 30] Door In Volume
      (if (Variables|Main|GetFunctionAsDoor)
        (Variables|Default|SetBackForward "NewEnumerator0")
        (Variables|Default|SetactiveState "NewEnumerator0")))))

(event EventBeginPlay
  (bind _platform (Variables|Components|GetPlatform))
  ;[1 1 1 1 25] Set Collision Channle
  (switch int (Variables|Default|GetNumber)
    (:Default
      (Development|PrintString "SET PLATFORM NUMBER!" true true "(R=1.000000,G=0.000000,B=0.130888,A=1.000000)"))
    (:0
      (Collision|SetCollisionObjectType _platform "ECC_GameTraceChannel1")
      (Variables|Default|SetPlats "ECC_GameTraceChannel1"))
    (:1
      (Collision|SetCollisionObjectType _platform "ECC_GameTraceChannel2")
      (Variables|Default|SetPlats "ECC_GameTraceChannel2"))
    (:2
      (Collision|SetCollisionObjectType _platform "ECC_GameTraceChannel3")
      (Variables|Default|SetPlats "ECC_GameTraceChannel3"))
    (:3
      (Collision|SetCollisionObjectType _platform "ECC_GameTraceChannel4")
      (Variables|Default|SetPlats "ECC_GameTraceChannel4"))
    (:4
      (Collision|SetCollisionObjectType _platform "ECC_GameTraceChannel5")
      (Variables|Default|SetPlats "ECC_GameTraceChannel5"))
    (:5
      (Development|PrintString "EXCEEDED VALUE RANGE FOR PLATFORMS! ADD NEW COLLISION CHANNELS " true true "(R=1.000000,G=0.000000,B=0.130888,A=1.000000)"))))

(event EventTick
  (params (DeltaSeconds :type Float%20%28single-precision%29))
  ;[0.3146 0.5071 1 1 50] Movement
  (CallFunction|Phase)
  (if (Utilities|Enum|Equal(Enum) (Variables|Default|GetactiveState) "NewEnumerator0")
    (if (Variables|Main|GetPressuerPlate)
      (if (Variables|Default|GetActivated)
        ;;[1 1 1] wait at a node
        (if (Variables|Default|GetWait) :!label _label
          (Utilities|FlowControl|Delay (Variables|Main|GetWaitTime))
          (Variables|Default|SetWait false))
        ;;[1 1 1] Interp from the begining of the spline to the end
        (CallFunction|FuncSetDistance)
        (CallFunction|FuncUpdatePosition)
        ;;[1 1 1] Change Direction
        (switch Utilities|FlowControl|Switch|SwitchonEnum_BackForward (Variables|Default|GetBackForward)
          (:NewEnumerator0
            (if (>= (Variables|Default|GetCurrDistance) (Variables|Default|GetDistance))
              (Variables|Default|SetBackForward "NewEnumerator1")
              (Variables|Default|SetWait true :!label _label_2)
              (if (Variables|Main|GetTeleport)
                (Variables|Default|SetCurrDistance 0.0)
                (CallFunction|FuncUpdatePosition))
              (if (Variables|Main|GetStopAtEnds)
                (Variables|Default|SetactiveState "NewEnumerator1"))))
          (:NewEnumerator1
            (if (<= (Variables|Default|GetCurrDistance) 0.0)
              (Variables|Default|SetBackForward "NewEnumerator0")
              (goto _label_2)))))
      (else
        (goto _label)))))

(fn ConstructionScript
  (bind _nodelocations (Variables|Default|GetNodeLocations))
  (bind _spline (Variables|Components|GetSpline))
  ;[1 0.5284 0.8962 1 30] SetMesh
  (Components|StaticMesh|SetStaticMesh (Variables|Components|GetPlatform) (Variables|Components|GetMesh))
  ;[0.2782 0.4586 1 1 30] Spline Lenght
  (Variables|Default|SetDistance (Spline|GetSplineLength (Variables|Components|GetSpline)))
  ;[0.3618 1 0.7219 1 30] Remove Unused Nodes
  (Utilities|Array|Clear _nodelocations)
  ;[0.5525 1 0.3047 1 30] Adding Nodes
  (for _index (range 0 (Spline|GetNumberOfSplinePoints _spline))
    (Utilities|Array|Add _nodelocations (Spline|GetDistanceAlongSplineatSplinePoint _spline _index))))

(fn FuncSetDistance
  (bind _distance (Variables|Default|GetDistance))
  (switch Utilities|FlowControl|Switch|SwitchonEnum_BackForward (Variables|Default|GetBackForward)
    (:NewEnumerator0
      (Variables|Default|SetCurrDistance (Math|Float|Clamp(Float) (+ (Math|Interpolation|FInterpTo 0.0 _distance 0.01 (* (/ (Variables|Main|GetForwardSpeed) _distance) 1e+03)) (Variables|Default|GetCurrDistance)) 0.0 _distance)))
    (:NewEnumerator1
      (Variables|Default|SetCurrDistance (Math|Float|Clamp(Float) (- (Variables|Default|GetCurrDistance) (Math|Interpolation|FInterpTo 0.0 _distance 0.01 (* (/ (Variables|Main|GetBackSpeed) _distance) 1e+03))) 0.0 _distance)))))

(fn FuncUpdatePosition
  (bind _currdistance (Variables|Default|GetCurrDistance))
  (bind _spline (Variables|Components|GetSpline))
  (if (Variables|Main|GetCanRotate)
    (Transformation|SetWorldLocationAndRotation (Variables|Components|GetPlatform) (Spline|GetLocationatDistanceAlongSpline _spline _currdistance "World") (Spline|GetRotationatDistanceAlongSpline _spline _currdistance "World") false false)
    (else
      (Transformation|SetWorldLocationAndRotation (Variables|Components|GetPlatform) (Spline|GetLocationatDistanceAlongSpline (Variables|Components|GetSpline) _currdistance "World") "0, 0, 0" false false))))