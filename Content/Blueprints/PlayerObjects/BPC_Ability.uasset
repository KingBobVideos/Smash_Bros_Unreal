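; Fighter component that owns a BP_Fighter's moveset and selects which move fires, in a platform-fighter style.
; AttachAbilities spawns one owned actor per move slot, from attacks and throws to dodges, taunts and extras.
; WitchAbility switches on AbilityType, then uses stick axes, Direction or facing to set the chosen actor Active, often updating the Attacks enum.
; EndAllNonChargedAbilities ends the fighter's other uncharged abilities, sparing the caller.
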(event Custom|witchAbility
  ;[0.2188 0.08816 0.07945 1 35] switch on ability type
  (switch Utilities|FlowControl|Switch|SwitchonEnum_abilityTypes (Variables|/Game/Blueprints/Characters/BP_Fighter.BP_Fighter_C|GetAbilityType (Variables|Default|GetParent))
    (:NewEnumerator1
      ;;[1 1 1] Comment
      (CallFunction|BasicAttack))
    (:NewEnumerator2
      (CallFunction|SpecialAttack))
    (:NewEnumerator3
      (CallFunction|AirAttacks))
    (:NewEnumerator4
      (CallFunction|Smashing))
    (:NewEnumerator7
      (CallFunction|Dodge))
    (:NewEnumerator8
      (CallFunction|Taunts))
    (:NewEnumerator10
      (CallFunction|Throw))
    (:NewEnumerator11
      (CallFunction|Prone))
    (:NewEnumerator12
      (Variables|/Game/Blueprints/Abilities/BP_BaseAbility.BP_BaseAbility_C|SetActive (Variables|Default|GetA_Grab) true))
    (:NewEnumerator6
      (Variables|/Game/Blueprints/Abilities/BP_BaseAbility.BP_BaseAbility_C|SetActive (Variables|Default|GetA_DashAttack) true))))

(event Custom|Dodge
  ;[0.4107 1 0.5581 1 35] Dodge
  (switch Utilities|FlowControl|Switch|SwitchonEnum_Direction (Variables|/Game/Blueprints/Characters/BP_Fighter.BP_Fighter_C|GetDirection (Variables|Default|GetParent))
    (:NewEnumerator2
      (Variables|/Game/Blueprints/Characters/BP_Fighter.BP_Fighter_C|SetAttacks (Variables|Default|GetParent) "NewEnumerator29")
      ;;[1 1 1 1 35] Activate Ability
      (Variables|/Game/Blueprints/Abilities/BP_BaseAbility.BP_BaseAbility_C|SetActive (Variables|Default|GetA_DodgeAir) true))
    (:NewEnumerator3
      (Variables|/Game/Blueprints/Characters/BP_Fighter.BP_Fighter_C|SetAttacks (Variables|Default|GetParent) "NewEnumerator28")
      (Variables|/Game/Blueprints/Abilities/BP_BaseAbility.BP_BaseAbility_C|SetActive (Variables|Default|GetA_DodgeSpot) true))
    (:NewEnumerator4
      (Variables|/Game/Blueprints/Characters/BP_Fighter.BP_Fighter_C|SetAttacks (Variables|Default|GetParent) "NewEnumerator30")
      (Variables|/Game/Blueprints/Abilities/BP_BaseAbility.BP_BaseAbility_C|SetActive (Variables|Default|GetA_DodgeBack) true))
    (:NewEnumerator5
      (Variables|/Game/Blueprints/Characters/BP_Fighter.BP_Fighter_C|SetAttacks (Variables|Default|GetParent) "NewEnumerator31")
      (Variables|/Game/Blueprints/Abilities/BP_BaseAbility.BP_BaseAbility_C|SetActive (Variables|Default|GetA_DodgeForward) true))))

(event Custom|AttachAbilities
  (bind (_returnvalue _parent) (Utilities|ParentTransform))
  (bind (_returnvalue_2 _parent_2) (Utilities|ParentTransform))
  (bind (_returnvalue_3 _parent_3) (Utilities|ParentTransform))
  (bind (_returnvalue_4 _parent_4) (Utilities|ParentTransform))
  (bind (_returnvalue_5 _parent_5) (Utilities|ParentTransform))
  (bind (_returnvalue_6 _parent_6) (Utilities|ParentTransform))
  (bind (_returnvalue_7 _parent_7) (Utilities|ParentTransform))
  (bind (_returnvalue_8 _parent_8) (Utilities|ParentTransform))
  (bind (_returnvalue_9 _parent_9) (Utilities|ParentTransform))
  (bind (_returnvalue_10 _parent_10) (Utilities|ParentTransform))
  (bind (_returnvalue_11 _parent_11) (Utilities|ParentTransform))
  (bind (_returnvalue_12 _parent_12) (Utilities|ParentTransform))
  (bind (_returnvalue_13 _parent_13) (Utilities|ParentTransform))
  (bind (_returnvalue_14 _parent_14) (Utilities|ParentTransform))
  (bind (_returnvalue_15 _parent_15) (Utilities|ParentTransform))
  (bind (_returnvalue_16 _parent_16) (Utilities|ParentTransform))
  (bind (_returnvalue_17 _parent_17) (Utilities|ParentTransform))
  (bind (_returnvalue_18 _parent_18) (Utilities|ParentTransform))
  (bind (_returnvalue_19 _parent_19) (Utilities|ParentTransform))
  (bind (_returnvalue_20 _parent_20) (Utilities|ParentTransform))
  (bind (_returnvalue_21 _parent_21) (Utilities|ParentTransform))
  (bind (_returnvalue_22 _parent_22) (Utilities|ParentTransform))
  (bind (_returnvalue_23 _parent_23) (Utilities|ParentTransform))
  (bind (_returnvalue_24 _parent_24) (Utilities|ParentTransform))
  (bind (_returnvalue_25 _parent_25) (Utilities|ParentTransform))
  (bind (_returnvalue_26 _parent_26) (Utilities|ParentTransform))
  (bind (_returnvalue_27 _parent_27) (Utilities|ParentTransform))
  (bind (_returnvalue_28 _parent_28) (Utilities|ParentTransform))
  (bind (_returnvalue_29 _parent_29) (Utilities|ParentTransform))
  (bind (_returnvalue_30 _parent_30) (Utilities|ParentTransform))
  (bind (_returnvalue_31 _parent_31) (Utilities|ParentTransform))
  (bind (_returnvalue_32 _parent_32) (Utilities|ParentTransform))
  (bind (_returnvalue_33 _parent_33) (Utilities|ParentTransform))
  (bind (_returnvalue_34 _parent_34) (Utilities|ParentTransform))
  (bind (_returnvalue_35 _parent_35) (Utilities|ParentTransform))
  (bind (_returnvalue_36 _parent_36) (Utilities|ParentTransform))
  (bind (_returnvalue_37 _parent_37) (Utilities|ParentTransform))
  (bind (_returnvalue_38 _parent_38) (Utilities|ParentTransform))
  (bind (_returnvalue_39 _parent_39) (Utilities|ParentTransform))
  (bind (_returnvalue_40 _parent_40) (Utilities|ParentTransform))
  (bind (_returnvalue_41 _parent_41) (Utilities|ParentTransform))
  (bind (_returnvalue_42 _parent_42) (Utilities|ParentTransform))
  (bind (_returnvalue_43 _parent_43) (Utilities|ParentTransform))
  (Utilities|FlowControl|Sequence
    (:then_0
      ;[0.6417 1 0.5249 1 40] Basic
      (bind _returnvalue_44 (Game|SpawnActorfromClass (Variables|Default|GetNeutral) _returnvalue_2 "AdjustIfPossibleButDontSpawnIfColliding" _parent_2 _parent_2 0))
      (Variables|Default|SetA_NeutralAttack _returnvalue_44)
      (bind _returnvalue_45 (Game|SpawnActorfromClass (Variables|Default|GetTiltUp) _returnvalue_4 "AdjustIfPossibleButDontSpawnIfColliding" _parent_4 _parent_4 0))
      (Variables|Default|SetA_TiltUp _returnvalue_45)
      (bind _returnvalue_46 (Game|SpawnActorfromClass (Variables|Default|GetTiltDown) _returnvalue_6 "AdjustIfPossibleButDontSpawnIfColliding" _parent_6 _parent_6 0))
      (Variables|Default|SetA_TiltDown _returnvalue_46)
      (bind _returnvalue_47 (Game|SpawnActorfromClass (Variables|Default|GetTiltSide) _returnvalue_7 "AdjustIfPossibleButDontSpawnIfColliding" _parent_7 _parent_7 0))
      (Variables|Default|SetA_TiltForward _returnvalue_47))
    (:then_1
      ;[0.2915 0.5109 1 1 40] Special
      (bind _returnvalue_48 (Game|SpawnActorfromClass (Variables|Default|GetSpecialNeutral) _returnvalue_11 "AdjustIfPossibleButDontSpawnIfColliding" _parent_11 _parent_11 0))
      (Variables|Default|SetA_SpecialNeutral _returnvalue_48)
      (bind _returnvalue_49 (Game|SpawnActorfromClass (Variables|Default|GetSpecialUP) _returnvalue_10 "AdjustIfPossibleButDontSpawnIfColliding" _parent_10 _parent_10 0))
      (Variables|Default|SetA_SpecialUp _returnvalue_49)
      (bind _returnvalue_50 (Game|SpawnActorfromClass (Variables|Default|GetSpecialDown) _returnvalue_9 "AdjustIfPossibleButDontSpawnIfColliding" _parent_9 _parent_9 0))
      (Variables|Default|SetA_SpecialDown _returnvalue_50)
      (bind _returnvalue_51 (Game|SpawnActorfromClass (Variables|Default|GetSpecialForward) _returnvalue_8 "AdjustIfPossibleButDontSpawnIfColliding" _parent_8 _parent_8 0))
      (Variables|Default|SetA_SpecialSide _returnvalue_51))
    (:then_2
      ;[1 0.3175 0.2578 1 40] Air
      (bind _returnvalue_52 (Game|SpawnActorfromClass (Variables|Default|GetAirNeutral) _returnvalue_12 "AdjustIfPossibleButDontSpawnIfColliding" _parent_12 _parent_12 0))
      (Variables|Default|SetA_AirNeutral _returnvalue_52)
      (bind _returnvalue_53 (Game|SpawnActorfromClass (Variables|Default|GetAirForward) _returnvalue_13 "AdjustIfPossibleButDontSpawnIfColliding" _parent_13 _parent_13 0))
      (Variables|Default|SetA_AirForward _returnvalue_53)
      (bind _returnvalue_54 (Game|SpawnActorfromClass (Variables|Default|GetAirBack) _returnvalue_14 "AdjustIfPossibleButDontSpawnIfColliding" _parent_14 _parent_14 0))
      (Variables|Default|SetA_AirBack _returnvalue_54)
      (bind _returnvalue_55 (Game|SpawnActorfromClass (Variables|Default|GetAirUp) _returnvalue_15 "AdjustIfPossibleButDontSpawnIfColliding" _parent_15 _parent_15 0))
      (Variables|Default|SetA_AirUp _returnvalue_55)
      (bind _returnvalue_56 (Game|SpawnActorfromClass (Variables|Default|GetAirDown) _returnvalue_16 "AdjustIfPossibleButDontSpawnIfColliding" _parent_16 _parent_16 0))
      (Variables|Default|SetA_AirDown _returnvalue_56))
    (:then_3
      ;[1 0.9929 0.3462 1 40] Smash
      (bind _returnvalue_57 (Game|SpawnActorfromClass (Variables|Default|GetSmashUp) _returnvalue_17 "AdjustIfPossibleButDontSpawnIfColliding" _parent_17 _parent_17 0))
      (Variables|Default|SetA_SmashUp _returnvalue_57)
      (bind _returnvalue_58 (Game|SpawnActorfromClass (Variables|Default|GetSmashForoward) _returnvalue_18 "AdjustIfPossibleButDontSpawnIfColliding" _parent_18 _parent_18 0))
      (Variables|Default|SetA_SmashForward _returnvalue_58)
      (bind _returnvalue_59 (Game|SpawnActorfromClass (Variables|Default|GetSmashDown) _returnvalue_19 "AdjustIfPossibleButDontSpawnIfColliding" _parent_19 _parent_19 0))
      (Variables|Default|SetA_SmashDown _returnvalue_59))
    (:then_4
      ;[1 0.2837 0.8702 1 40] Grab And Trow
      (bind _returnvalue_60 (Game|SpawnActorfromClass (Variables|Default|GetGrab) _returnvalue_20 "AdjustIfPossibleButDontSpawnIfColliding" _parent_20 _parent_20 0))
      (Variables|Default|SetA_Grab _returnvalue_60)
      (bind _returnvalue_61 (Game|SpawnActorfromClass (Variables|Default|GetPummle) _returnvalue_21 "AdjustIfPossibleButDontSpawnIfColliding" _parent_21 _parent_21 0))
      (Variables|Default|SetA_Pummel _returnvalue_61)
      (bind _returnvalue_62 (Game|SpawnActorfromClass (Variables|Default|GetThrowUP) _returnvalue_22 "AdjustIfPossibleButDontSpawnIfColliding" _parent_22 _parent_22 0))
      (Variables|Default|SetA_ThrowUP _returnvalue_62)
      (bind _returnvalue_63 (Game|SpawnActorfromClass (Variables|Default|GetThrowDown) _returnvalue_24 "AdjustIfPossibleButDontSpawnIfColliding" _parent_24 _parent_24 0))
      (Variables|Default|SetA_ThrowDown _returnvalue_63)
      (bind _returnvalue_64 (Game|SpawnActorfromClass (Variables|Default|GetThrowBack) _returnvalue_25 "AdjustIfPossibleButDontSpawnIfColliding" _parent_25 _parent_25 0))
      (Variables|Default|SetA_ThrowBackward _returnvalue_64)
      (bind _returnvalue_65 (Game|SpawnActorfromClass (Variables|Default|GetThrowForward) _returnvalue_26 "AdjustIfPossibleButDontSpawnIfColliding" _parent_26 _parent_26 0))
      (Variables|Default|SetA_ThrowForward _returnvalue_65))
    (:then_5
      ;[1 0.5683 0.2174 1 40] Dodge
      (bind _returnvalue_66 (Game|SpawnActorfromClass (Variables|Default|GetDodgeAir) _returnvalue_27 "AdjustIfPossibleButDontSpawnIfColliding" _parent_27 _parent_27 0))
      (Variables|Default|SetA_DodgeAir _returnvalue_66)
      (bind _returnvalue_67 (Game|SpawnActorfromClass (Variables|Default|GetDodgeBack) _returnvalue_28 "AdjustIfPossibleButDontSpawnIfColliding" _parent_28 _parent_28 0))
      (Variables|Default|SetA_DodgeBack _returnvalue_67)
      (bind _returnvalue_68 (Game|SpawnActorfromClass (Variables|Default|GetDodgeForward) _returnvalue_29 "AdjustIfPossibleButDontSpawnIfColliding" _parent_29 _parent_29 0))
      (Variables|Default|SetA_DodgeForward _returnvalue_68)
      (bind _returnvalue_69 (Game|SpawnActorfromClass (Variables|Default|GetDodgeSpot) _returnvalue_30 "AdjustIfPossibleButDontSpawnIfColliding" _parent_30 _parent_30 0))
      (Variables|Default|SetA_DodgeSpot _returnvalue_69))
    (:then_6
      ;[0.3645 1 0.9901 1 40] Taunts
      (bind _returnvalue_70 (Game|SpawnActorfromClass (Variables|Default|GetTauntUp) _returnvalue_31 "AdjustIfPossibleButDontSpawnIfColliding" _parent_31 _parent_31 0))
      (Variables|Default|SetA_TauntUp _returnvalue_70)
      (bind _returnvalue_71 (Game|SpawnActorfromClass (Variables|Default|GetTauntDown) _returnvalue_32 "AdjustIfPossibleButDontSpawnIfColliding" _parent_32 _parent_32 0))
      (Variables|Default|SetA_TauntDown _returnvalue_71)
      (bind _returnvalue_72 (Game|SpawnActorfromClass (Variables|Default|GetTauntLeft) _returnvalue_33 "AdjustIfPossibleButDontSpawnIfColliding" _parent_33 _parent_33 0))
      (Variables|Default|SetA_TauntLeft _returnvalue_72)
      (bind _returnvalue_73 (Game|SpawnActorfromClass (Variables|Default|GetTauntRight) _returnvalue_34 "AdjustIfPossibleButDontSpawnIfColliding" _parent_34 _parent_34 0))
      (Variables|Default|SetA_TauntRight _returnvalue_73)
      (bind _returnvalue_74 (Game|SpawnActorfromClass (Variables|Default|GetLevelIntro) _returnvalue_35 "AdjustIfPossibleButDontSpawnIfColliding" _parent_35 _parent_35 0))
      (Variables|Default|SetA_LevelIntro _returnvalue_74))
    (:then_7
      ;[1 1 1 1 40] Other
      (bind _returnvalue_75 (Game|SpawnActorfromClass (Variables|Default|GetDashAttack) _returnvalue_36 "AdjustIfPossibleButDontSpawnIfColliding" _parent_36 _parent_36 0))
      (Variables|Default|SetA_DashAttack _returnvalue_75)
      (bind _returnvalue_76 (Game|SpawnActorfromClass (Variables|Default|GetLedgeAttack) _returnvalue_37 "AdjustIfPossibleButDontSpawnIfColliding" _parent_37 _parent_37 0))
      (Variables|Default|SetA_LedgeAttack _returnvalue_76)
      (bind _returnvalue_77 (Game|SpawnActorfromClass (Variables|Default|GetProneAttack) _returnvalue_38 "AdjustIfPossibleButDontSpawnIfColliding" _parent_38 _parent_38 0))
      (Variables|Default|SetA_ProneAttack _returnvalue_77)
      (bind _returnvalue_78 (Game|SpawnActorfromClass (Variables|Default|GetProneStand) _returnvalue_39 "AdjustIfPossibleButDontSpawnIfColliding" _parent_39 _parent_39 0))
      (Variables|Default|SetA_ProneStand _returnvalue_78)
      (bind _returnvalue_79 (Game|SpawnActorfromClass (Variables|Default|GetSuper) _returnvalue_40 "AdjustIfPossibleButDontSpawnIfColliding" _parent_40 _parent_40 0))
      (Variables|Default|SetA_Super _returnvalue_79)
      (bind _returnvalue_80 (Game|SpawnActorfromClass (Variables|Default|GetLedge) _returnvalue_41 "AdjustIfPossibleButDontSpawnIfColliding" _parent_41 _parent_41 0))
      (Variables|Default|SetA_Ledge _returnvalue_80)
      (bind _returnvalue_81 (Game|SpawnActorfromClass (Variables|Default|GetRespawn) _returnvalue_42 "AdjustIfPossibleButDontSpawnIfColliding" _parent_42 _parent_42 0))
      (Variables|Default|SetA_respawn _returnvalue_81)
      (bind _returnvalue_82 (Game|SpawnActorfromClass (Variables|Default|GetItems) _returnvalue_43 "AdjustIfPossibleButDontSpawnIfColliding" _parent_43 _parent_43 0))
      (Variables|Default|SetA_Item _returnvalue_82))
    (:then_8
      ;[0.09896 0.06987 0.03885 1 30] Extra ability slots
      (bind _returnvalue_83 (Game|SpawnActorfromClass (Variables|Default|GetExtra_01) _returnvalue "AdjustIfPossibleButDontSpawnIfColliding" _parent _parent 0))
      (Variables|Default|SetA_Extra_01 _returnvalue_83)
      (bind _returnvalue_84 (Game|SpawnActorfromClass (Variables|Default|GetExtra_02) _returnvalue_3 "AdjustIfPossibleButDontSpawnIfColliding" _parent_3 _parent_3 0))
      (Variables|Default|SetA_Extra_02 _returnvalue_84)
      (bind _returnvalue_85 (Game|SpawnActorfromClass (Variables|Default|GetExtra_03) _returnvalue_5 "AdjustIfPossibleButDontSpawnIfColliding" _parent_5 _parent_5 0))
      (Variables|Default|SetA_Extra_03 _returnvalue_85)
      (bind _returnvalue_86 (Game|SpawnActorfromClass (Variables|Default|GetExtra_04) _returnvalue_23 "AdjustIfPossibleButDontSpawnIfColliding" _parent_23 _parent_23 0))
      (Variables|Default|SetA_Extra_04 _returnvalue_86))))

(event Custom|Extras
  (params (Selection :type Integer))
  ;[1 1 1 1 30] Extras
  (switch int Selection
    (:0
      (Variables|/Game/Blueprints/Abilities/BP_BaseAbility.BP_BaseAbility_C|SetActive (Variables|Default|GetA_Extra_01) true))
    (:1
      (Variables|/Game/Blueprints/Abilities/BP_BaseAbility.BP_BaseAbility_C|SetActive (Variables|Default|GetA_Extra_02) true))
    (:2
      (Variables|/Game/Blueprints/Abilities/BP_BaseAbility.BP_BaseAbility_C|SetActive (Variables|Default|GetA_Extra_03) true))
    (:3
      (Variables|/Game/Blueprints/Abilities/BP_BaseAbility.BP_BaseAbility_C|SetActive (Variables|Default|GetA_Extra_04) true))))

(event Custom|Prone
  ;[0.4554 0.4034 1 1 35] Prone
  (switch Utilities|FlowControl|Switch|SwitchonEnum_Direction (Variables|/Game/Blueprints/Characters/BP_Fighter.BP_Fighter_C|GetDirection (Variables|Default|GetParent))
    (:NewEnumerator2
      ;;[1 1 1 1 35] Activate Ability
      (Variables|/Game/Blueprints/Abilities/BP_BaseAbility.BP_BaseAbility_C|SetActive (Variables|Default|GetA_ProneStand) true))
    (:NewEnumerator3
      (Variables|/Game/Blueprints/Abilities/BP_BaseAbility.BP_BaseAbility_C|SetActive (Variables|Default|GetA_ProneAttack) true))))

(event Custom|SpecialAttack
  (bind _parent (Variables|Default|GetParent))
  (bind _parent_2 (Variables|Default|GetParent))
  (bind _leftright (Variables|/Game/Blueprints/Characters/BP_Fighter.BP_Fighter_C|GetLeftRight _parent_2))
  (bind _updown (Variables|/Game/Blueprints/Characters/BP_Fighter.BP_Fighter_C|GetUpDown _parent))
  ;[1 0.5026 0.4328 1 35] Set Special Attack
  (if (>= _updown 0.2)
    (Variables|/Game/Blueprints/Characters/BP_Fighter.BP_Fighter_C|SetAttacks (Variables|Default|GetParent) "NewEnumerator10")
    ;;[1 1 1 1 35] Activate Ability
    (Variables|/Game/Blueprints/Abilities/BP_BaseAbility.BP_BaseAbility_C|SetActive (Variables|Default|GetA_SpecialUp) true)
    (elif (<= _updown -0.2)
      (Variables|/Game/Blueprints/Characters/BP_Fighter.BP_Fighter_C|SetAttacks (Variables|Default|GetParent) "NewEnumerator11")
      (Variables|/Game/Blueprints/Abilities/BP_BaseAbility.BP_BaseAbility_C|SetActive (Variables|Default|GetA_SpecialDown) true)
      (elif (>= _leftright 0.2)
        (Variables|/Game/Blueprints/Characters/BP_Fighter.BP_Fighter_C|SetAttacks (Variables|Default|GetParent) "NewEnumerator12" :!label _label)
        (Variables|/Game/Blueprints/Abilities/BP_BaseAbility.BP_BaseAbility_C|SetActive (Variables|Default|GetA_SpecialSide) true)
        (elif (<= _leftright -0.2)
          (goto _label)
          (else
            (Variables|/Game/Blueprints/Characters/BP_Fighter.BP_Fighter_C|SetAttacks (Variables|Default|GetParent) "NewEnumerator26")
            (Variables|/Game/Blueprints/Abilities/BP_BaseAbility.BP_BaseAbility_C|SetActive (Variables|Default|GetA_SpecialNeutral) true)))))))

(event Custom|Taunts
  ;[0.4054 1 0.9701 1 35] taunts
  (switch Utilities|FlowControl|Switch|SwitchonEnum_Direction (Variables|/Game/Blueprints/Characters/BP_Fighter.BP_Fighter_C|GetDirection (Variables|Default|GetParent))
    (:NewEnumerator2
      ;;[1 1 1 1 35] Activate Ability
      (Variables|/Game/Blueprints/Abilities/BP_BaseAbility.BP_BaseAbility_C|SetActive (Variables|Default|GetA_TauntUp) true))
    (:NewEnumerator3
      (Variables|/Game/Blueprints/Abilities/BP_BaseAbility.BP_BaseAbility_C|SetActive (Variables|Default|GetA_TauntDown) true))
    (:NewEnumerator4
      (Variables|/Game/Blueprints/Abilities/BP_BaseAbility.BP_BaseAbility_C|SetActive (Variables|Default|GetA_TauntLeft) true))
    (:NewEnumerator5
      (Variables|/Game/Blueprints/Abilities/BP_BaseAbility.BP_BaseAbility_C|SetActive (Variables|Default|GetA_TauntRight) true))))

(event Custom|OnLedge)

(event Custom|Throw
  ;[0.2874 0.5502 1 1 35] Throwing
  (switch Utilities|FlowControl|Switch|SwitchonEnum_Direction (Variables|/Game/Blueprints/Characters/BP_Fighter.BP_Fighter_C|GetDirection (Variables|Default|GetParent))
    (:NewEnumerator2
      ;;[1 1 1 1 35] Activate Ability
      (Variables|/Game/Blueprints/Abilities/BP_BaseAbility.BP_BaseAbility_C|SetActive (Variables|Default|GetA_ThrowUP) true))
    (:NewEnumerator3
      (Variables|/Game/Blueprints/Abilities/BP_BaseAbility.BP_BaseAbility_C|SetActive (Variables|Default|GetA_ThrowDown) true))
    (:NewEnumerator4
      (Variables|/Game/Blueprints/Abilities/BP_BaseAbility.BP_BaseAbility_C|SetActive (Variables|Default|GetA_ThrowBackward) true))
    (:NewEnumerator5
      (Variables|/Game/Blueprints/Abilities/BP_BaseAbility.BP_BaseAbility_C|SetActive (Variables|Default|GetA_ThrowForward) true))))

(event Custom|BasicAttack
  (bind _a_tiltup (Variables|Default|GetA_TiltUp))
  (bind _a_neutralattack (Variables|Default|GetA_NeutralAttack))
  (bind _parent (Variables|Default|GetParent))
  (bind _parent_2 (Variables|Default|GetParent))
  (bind _updown (Variables|/Game/Blueprints/Characters/BP_Fighter.BP_Fighter_C|GetUpDown _parent))
  (bind _leftright (Variables|/Game/Blueprints/Characters/BP_Fighter.BP_Fighter_C|GetLeftRight _parent_2))
  ;[1 0.4314 0.7009 1 35] Set Basic Attack
  (if (>= _updown 0.2)
    (Variables|/Game/Blueprints/Characters/BP_Fighter.BP_Fighter_C|SetAttacks (Variables|Default|GetParent) "NewEnumerator0")
    ;;[1 1 1 1 35] Activate Ability
    (Utilities|IsValid _a_tiltup
      (:Is%20Valid
        (Variables|/Game/Blueprints/Abilities/BP_BaseAbility.BP_BaseAbility_C|SetActive _a_tiltup true)))
    (elif (<= _updown -0.2)
      (Variables|/Game/Blueprints/Characters/BP_Fighter.BP_Fighter_C|SetAttacks (Variables|Default|GetParent) "NewEnumerator1")
      (Variables|/Game/Blueprints/Abilities/BP_BaseAbility.BP_BaseAbility_C|SetActive (Variables|Default|GetA_TiltDown) true)
      (elif (>= _leftright 0.2)
        (Variables|/Game/Blueprints/Characters/BP_Fighter.BP_Fighter_C|SetAttacks (Variables|Default|GetParent) "NewEnumerator2" :!label _label)
        (Variables|/Game/Blueprints/Abilities/BP_BaseAbility.BP_BaseAbility_C|SetActive (Variables|Default|GetA_TiltForward) true)
        (elif (<= _leftright -0.2)
          (goto _label)
          (else
            (Variables|/Game/Blueprints/Characters/BP_Fighter.BP_Fighter_C|SetAttacks (Variables|Default|GetParent) "NewEnumerator4")
            (Utilities|IsValid _a_neutralattack
              (:Is%20Valid
                (Variables|/Game/Blueprints/Abilities/BP_BaseAbility.BP_BaseAbility_C|SetActive _a_neutralattack true)))))))))

(event Custom|EndAllNonChargedAbilities
  (params (Caller :type BP%20Base%20Ability%20Object%20Reference))
  (bind _outactors (Actor|GetAllActorsOfClass "/Game/Blueprints/Abilities/BP_BaseAbility.BP_BaseAbility_C"))
  (for _array_element _outactors
    (if (Math|Boolean|ANDBoolean (== (Variables|/Game/Blueprints/Abilities/BP_BaseAbility.BP_BaseAbility_C|GetParent _array_element) (Variables|Default|GetParent)) (== (Variables|/Game/Blueprints/Abilities/BP_BaseAbility.BP_BaseAbility_C|GetChargeLevel _array_element) 0.0) (!= Caller _array_element))
      (Default|EndAbility _array_element))))

(event Custom|Respawning
  ;[0.2969 0.2969 0.2969 1 35] Respawn
  (if (Utilities|Enum|Equal(Enum) (Variables|/Game/Blueprints/Characters/BP_Fighter.BP_Fighter_C|GetStates (Variables|Default|GetParent)) "NewEnumerator9")
    (Variables|/Game/Blueprints/Abilities/BP_BaseAbility.BP_BaseAbility_C|SetActive (Variables|Default|GetA_respawn) true)))

(event Custom|Smashing
  ;[0.7963 1 0.3524 1 35] Set Smash Attacks
  (switch Utilities|FlowControl|Switch|SwitchonEnum_Direction (Variables|/Game/Blueprints/Characters/BP_Fighter.BP_Fighter_C|GetDirection (Variables|Default|GetParent))
    (:NewEnumerator2
      (Variables|/Game/Blueprints/Characters/BP_Fighter.BP_Fighter_C|SetAttacks (Variables|Default|GetParent) "NewEnumerator14")
      ;;[1 1 1 1 35] Activate Ability
      (Variables|/Game/Blueprints/Abilities/BP_BaseAbility.BP_BaseAbility_C|SetActive (Variables|Default|GetA_SmashUp) true))
    (:NewEnumerator3
      (Variables|/Game/Blueprints/Characters/BP_Fighter.BP_Fighter_C|SetAttacks (Variables|Default|GetParent) "NewEnumerator15")
      (Variables|/Game/Blueprints/Abilities/BP_BaseAbility.BP_BaseAbility_C|SetActive (Variables|Default|GetA_SmashDown) true))
    (:NewEnumerator5
      (Variables|/Game/Blueprints/Characters/BP_Fighter.BP_Fighter_C|SetAttacks (Variables|Default|GetParent) "NewEnumerator12")
      (Variables|/Game/Blueprints/Abilities/BP_BaseAbility.BP_BaseAbility_C|SetActive (Variables|Default|GetA_SmashForward) true))))

(event Custom|AirAttacks
  (bind _parent (Variables|Default|GetParent))
  (bind _parent_2 (Variables|Default|GetParent))
  (bind _faceing (Variables|/Game/Blueprints/Characters/BP_Fighter.BP_Fighter_C|GetFaceing _parent_2))
  (bind _updown (Variables|/Game/Blueprints/Characters/BP_Fighter.BP_Fighter_C|GetUpDown _parent))
  (bind _leftright (Variables|/Game/Blueprints/Characters/BP_Fighter.BP_Fighter_C|GetLeftRight _parent_2))
  ;[1 0.8374 0.4904 1 35] Set Air Attack
  (if (>= _updown 0.5)
    (Variables|/Game/Blueprints/Characters/BP_Fighter.BP_Fighter_C|SetAttacks (Variables|Default|GetParent) "NewEnumerator5")
    ;;[1 1 1 1 35] Activate Ability
    (Variables|/Game/Blueprints/Abilities/BP_BaseAbility.BP_BaseAbility_C|SetActive (Variables|Default|GetA_AirUp) true)
    (elif (<= _updown -0.5)
      (Variables|/Game/Blueprints/Characters/BP_Fighter.BP_Fighter_C|SetAttacks (Variables|Default|GetParent) "NewEnumerator6")
      (Variables|/Game/Blueprints/Abilities/BP_BaseAbility.BP_BaseAbility_C|SetActive (Variables|Default|GetA_AirDown) true)
      (elif (>= _leftright 0.5)
        (switch Utilities|FlowControl|Switch|SwitchonEnum_faceing _faceing
          (:NewEnumerator0
            (Variables|/Game/Blueprints/Characters/BP_Fighter.BP_Fighter_C|SetAttacks (Variables|Default|GetParent) "NewEnumerator7" :!label _label)
            (Variables|/Game/Blueprints/Abilities/BP_BaseAbility.BP_BaseAbility_C|SetActive (Variables|Default|GetA_AirBack) true))
          (:NewEnumerator1
            (Variables|/Game/Blueprints/Characters/BP_Fighter.BP_Fighter_C|SetAttacks (Variables|Default|GetParent) "NewEnumerator8" :!label _label_2)
            (Variables|/Game/Blueprints/Abilities/BP_BaseAbility.BP_BaseAbility_C|SetActive (Variables|Default|GetA_AirForward) true)))
        (elif (<= _leftright -0.5)
          (switch Utilities|FlowControl|Switch|SwitchonEnum_faceing _faceing
            (:NewEnumerator0
              (goto _label_2))
            (:NewEnumerator1
              (goto _label)))
          (else
            (Variables|/Game/Blueprints/Characters/BP_Fighter.BP_Fighter_C|SetAttacks (Variables|Default|GetParent) "NewEnumerator5")
            (Variables|/Game/Blueprints/Abilities/BP_BaseAbility.BP_BaseAbility_C|SetActive (Variables|Default|GetA_AirNeutral) true)))))))

(event EventTick
  (params (DeltaSeconds :type Float%20%28single-precision%29))
  (bind _parent (Variables|Default|GetParent))
  ;[0.7083 0.8171 1 1 30] Comment
  (if (and (Utilities|Enum|Equal(Enum) (Variables|/Game/Blueprints/Characters/BP_Fighter.BP_Fighter_C|GetStates _parent) "NewEnumerator18") (Utilities|Enum|Equal(Enum) (Variables|/Game/Blueprints/Characters/BP_Fighter.BP_Fighter_C|GetAttacks _parent) "NewEnumerator27"))
    (CallFunction|WitchAbility)))

(event EventBeginPlay
  ;[0.6392 0.8958 0.7227 1 35] GetOwner
  (bind _asbp_fighter (Utilities|Casting|CastToBP_Fighter (Components|GetOwner)))
  (Variables|Default|SetParent _asbp_fighter))