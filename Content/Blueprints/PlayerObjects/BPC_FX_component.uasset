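; Fighter effects component that shows a smoke trail on its owning BP_Fighter during two specific fighter states.
; Each tick it checks the owner's state and, through a DoOnce, attaches one smoke trail emitter to the mesh's pelvis, storing it on the fighter.
; In any other state it ends the trails of a valid stored emitter and resets the DoOnce, without destroying the component.
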(event EventBeginPlay
  (bind _asbp_fighter (Utilities|Casting|CastToBP_Fighter (Components|GetOwner)))
  (Variables|Default|SetParent _asbp_fighter))

(event EventTick
  (params (DeltaSeconds :type Float%20%28single-precision%29))
  (bind _parent (Variables|Default|GetParent))
  (bind _states (Variables|/Game/Blueprints/Characters/BP_Fighter.BP_Fighter_C|GetStates _parent))
  (if (or (Utilities|Enum|Equal(Enum) _states "NewEnumerator6") (Utilities|Enum|Equal(Enum) _states "NewEnumerator13"))
    (Utilities|FlowControl|DoOnce false :!label _label
      (:Completed
        (bind _returnvalue (Effects|SpawnEmitterAttached "/Game/Assets/FX/Particles/P_SmokeTrail.P_SmokeTrail" (Variables|/Script/Engine.Character|GetMesh (Variables|Default|GetParent)) "pelvis" "0, 0, 0" "0, 0, 0" "1.000000,1.000000,1.000000" "SnapToTarget" false))
        (Variables|/Game/Blueprints/Characters/BP_Fighter.BP_Fighter_C|SetSmoke (Variables|Default|GetParent) _returnvalue)))
    (else
      (Utilities|IsValid (Variables|/Game/Blueprints/Characters/BP_Fighter.BP_Fighter_C|GetSmoke (Variables|Default|GetParent))
        (:Is%20Valid
          (Effects|Particles|Trails|EndTrails (Variables|/Game/Blueprints/Characters/BP_Fighter.BP_Fighter_C|GetSmoke (Variables|Default|GetParent)))
          (goto _label Reset))))))