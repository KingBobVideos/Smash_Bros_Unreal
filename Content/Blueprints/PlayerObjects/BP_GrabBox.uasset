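; BP_GrabBox is a short-lived grab hitbox that lets one fighter seize another.
; Construction keeps a sphere or box collider; overlapping another owner's grab box destroys it, and it expires shortly after spawning.
; The first valid fighter collision triggers SetGrabState through authority-split server/client events.
; That plays hit effects, sets both fighters' states, turns the target toward the grabber, attaches it to the hand socket, then destroys the box.
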(event OnComponentBeginOverlap(Box)
  (params (OverlappedComponent :type Primitive%20Component%20Object%20Reference) (OtherActor :type Actor%20Object%20Reference) (OtherComp :type Primitive%20Component%20Object%20Reference) (OtherBodyIndex :type Integer) (bFromSweep :type Boolean) (SweepResult :type Hit%20Result%20Structure%20%28by%20ref%29))
  ;[0.908 1 0.3269 1 30] Overlap
  (CallFunction|OverlapOtherGrabBox OtherActor)
  (bind _asbp_fighter (Utilities|OverlapConditions OtherActor OtherComp)
    (:true
      (CallFunction|GrabStates _asbp_fighter))))

(event OnComponentBeginOverlap(Sphere)
  (params (OverlappedComponent :type Primitive%20Component%20Object%20Reference) (OtherActor :type Actor%20Object%20Reference) (OtherComp :type Primitive%20Component%20Object%20Reference) (OtherBodyIndex :type Integer) (bFromSweep :type Boolean) (SweepResult :type Hit%20Result%20Structure%20%28by%20ref%29))
  ;[0.908 1 0.3269 1 30] Overlap
  (CallFunction|OverlapOtherGrabBox OtherActor)
  (bind _asbp_fighter (Utilities|OverlapConditions OtherActor OtherComp)
    (:true
      (CallFunction|GrabStates _asbp_fighter))))

(event Custom|SetGrabStateClients
  (params (Target :type BP%20Fighter%20Object%20Reference) (Parent :type BP%20Fighter%20Object%20Reference) (Target1 :type BP%20Grab%20Box%20Object%20Reference))
  ;[0.3441 0.6427 1 1 30] Set Grab State
  (CallFunction|SetGrabState Target Parent Target1)
  (Utilities|FlowControl|Delay 0.01)
  (Actor|DestroyActor))

(event Custom|SetGrabStateServer
  (params (Target :type BP%20Fighter%20Object%20Reference) (Parent :type BP%20Fighter%20Object%20Reference) (Target1 :type BP%20Grab%20Box%20Object%20Reference))
  ;[0.3441 0.6427 1 1 30] Set Grab State
  (CallFunction|SetGrabState Target Parent Target1)
  (Utilities|FlowControl|Delay 0.01)
  (Actor|DestroyActor))

(event Custom|DeactivateEvent
  ;[1 0.1875 0.1875 1 30] Destory Self
  (Actor|DestroyActor))

(event Custom|GrabStates
  (params (Target :type BP%20Fighter%20Object%20Reference))
  (bind _self self)
  (bind _parent (Variables|Default|GetParent))
  ;[0.3441 0.6427 1 1 30] Set Grab State
  (Utilities|FlowControl|DoOnce false
    (:Completed
      (bind _output_get (Variables|Default|SetTarget Target))
      (Networking|SwitchHasAuthority
        (:Authority
          (CallFunction|SetGrabStateServer _output_get _parent _self))
        (:Remote
          (CallFunction|SetGrabStateClients _output_get _parent _self))))))

(event Custom|Flinch
  ;[1 0.1875 0.1875 1 30] Destory Self
  (Actor|DestroyActor))

(event EventBeginPlay
  ;[1 0.1875 0.1875 1 30] Destory Self
  (Utilities|FlowControl|Delay 0.2)
  (Actor|DestroyActor))

(fn ConstructionScript
  (switch Utilities|FlowControl|Switch|SwitchonEnum_shape (Variables|Default|GetCollisionShape)
    (:NewEnumerator0
      (Components|DestroyComponent (Variables|Default|GetBox)))
    (:NewEnumerator1
      (Components|DestroyComponent (Variables|Default|GetSphere)))))

(fn OverlapOtherGrabBox
  (params (Object :type Object%20Object%20Reference))
  (bind _asbp_grab_box (Utilities|Casting|CastToBP_GrabBox Object))
  (if (!= (Components|GetOwner _asbp_grab_box) (Components|GetOwner))
    (CallFunction|Flinch)))

(fn SetGrabState
  (params (Target :type BP%20Fighter%20Object%20Reference) (Parent :type BP%20Fighter%20Object%20Reference) (Target1 :type BP%20Grab%20Box%20Object%20Reference))
  (bind _handr (Variables|/Game/Blueprints/Characters/BP_Fighter.BP_Fighter_C|GetHandR Parent))
  (bind _rootcomponent (Variables|/Script/Engine.Actor|GetRootComponent Target1))
  (bind _returnvalue (Transformation|GetWorldLocation _handr))
  (bind _returnvalue_2 (Transformation|GetWorldLocation _rootcomponent))
  (bind (_x _y _z) (Math|Vector|BreakVector _returnvalue))
  (bind _returnvalue_3 (Math|Vector|MakeVector 4e+01 _y _z))
  (Audio|PlaySoundatLocation Target1 (Variables|Default|GetHitSound) _returnvalue_2 "0, 0, 0" 1.0 1.0 0.0 0 0 0)
  (Effects|SpawnEmitteratLocation Target1 (Variables|Default|GetHitParticel) _returnvalue_2)
  (Variables|/Game/Blueprints/Characters/BP_Fighter.BP_Fighter_C|SetStates Parent "NewEnumerator22")
  (Variables|/Game/Blueprints/Characters/BP_Fighter.BP_Fighter_C|SetStates Target "NewEnumerator21")
  (Variables|/Game/Blueprints/Characters/BP_Fighter.BP_Fighter_C|SetAttachTimer Parent 0.0)
  (switch Utilities|FlowControl|Switch|SwitchonEnum_faceing (Variables|/Game/Blueprints/Characters/BP_Fighter.BP_Fighter_C|GetFaceing Parent)
    (:NewEnumerator0
      (Variables|/Game/Blueprints/Characters/BP_Fighter.BP_Fighter_C|SetFaceing Target "NewEnumerator1")
      (Transformation|SetActorLocation Target _returnvalue_3 false false))
    (:NewEnumerator1
      (Variables|/Game/Blueprints/Characters/BP_Fighter.BP_Fighter_C|SetFaceing Target "NewEnumerator0")
      (Transformation|SetActorLocation Target _returnvalue_3 false false)))
  (if (!= Target Parent)
    (Transformation|AttachActorToActor Target Parent "hand_rSocket" "KeepWorld" "KeepWorld" "KeepWorld" true)
    (Variables|/Game/Blueprints/Characters/BP_Fighter.BP_Fighter_C|SetAttachedTo Target Parent)
    (Variables|/Game/Blueprints/Characters/BP_Fighter.BP_Fighter_C|SetAttachedTo Parent Target)))