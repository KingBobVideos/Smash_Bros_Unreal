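; BP_damagerInfo is an editor-time marker that previews a damage collision shape and its placement within a parent BP_BaseAbility.
; Its construction script finds the parent ability, records its transform and writes the relative location to a text label.
; It shows the sphere or box by CollisionShape, hiding everything when the ability filters to a different attack stage than its SetNo.
; At runtime it destroys itself just after BeginPlay.
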(event EventBeginPlay
  (Utilities|FlowControl|Delay 0.01)
  (Actor|DestroyActor))

(fn ConstructionScript
  (bind _scene (Variables|Default|GetScene))
  (bind _location (Variables|Default|GetLocation))
  (bind _boxscale (Variables|Default|Getboxscale))
  (bind _box (Variables|Default|GetBox))
  (bind _sphere (Variables|Default|GetSphere))
  (bind _relativelocation (Variables|/Script/Engine.SceneComponent|GetRelativeLocation _scene))
  (bind _outactors (Actor|GetAllActorsOfClass "/Game/Blueprints/Abilities/BP_BaseAbility.BP_BaseAbility_C"))
  (for _array_element _outactors
    (if (== _array_element (Actor|GetParentActor))
      (Variables|Default|Setability _array_element)))
  (Rendering|Components|TextRender|SetText (Variables|Default|GetLocation) (Utilities|Text|ToText(String) _relativelocation))
  (Variables|Transform|SetLocation+ _relativelocation)
  (Variables|Transform|SetScale (Transformation|GetActorScale3D))
  (Variables|Transform|SetRotation (Transformation|GetActorRotation))
  (if (Variables|/Game/Blueprints/Abilities/BP_BaseAbility.BP_BaseAbility_C|GetShowAttackStageOnly (Variables|Default|Getability))
    (if (== (Variables|/Game/Blueprints/Abilities/BP_BaseAbility.BP_BaseAbility_C|GetEditorAttackStage (Variables|Default|Getability)) (Variables|Main|GetSetNo))
      (switch Utilities|FlowControl|Switch|SwitchonEnum_shape (Variables|Main|GetCollisionShape) :!label _label
        (:NewEnumerator0
          (Rendering|SetVisibility _location true false)
          (Rendering|SetVisibility _boxscale true false)
          (Rendering|SetVisibility _sphere true false)
          (Rendering|SetVisibility _box false false))
        (:NewEnumerator1
          (Rendering|SetVisibility _location true false)
          (Rendering|SetVisibility _boxscale true false)
          (Rendering|SetVisibility _sphere false false)
          (Rendering|SetVisibility _box true false)))
      (else
        (Rendering|SetVisibility (Variables|Default|GetLocation) false false)
        (Rendering|SetVisibility (Variables|Default|Getboxscale) false false)
        (Rendering|SetVisibility (Variables|Default|GetSphere) false false)
        (Rendering|SetVisibility (Variables|Default|GetBox) false false)))
    (else
      (goto _label))))