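; BP_respwan is a respawn platform that glides down to a target height and removes itself after a few seconds.
; It also self-destructs shortly after its owning BP_Fighter gives left/right input or enters a particular state.
; Every Tick, Phase loops over all fighters, making each capsule block the Plats channel only when its feet are above the platform and it is not phasing, creating one-way collision.
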(event Custom|Leave
  ;[1 1 1] LeavePlatform
  (bind _asbp_fighter (Utilities|Casting|CastToBP_Fighter (Components|GetOwner)))
  (if (or (!= (Variables|/Game/Blueprints/Characters/BP_Fighter.BP_Fighter_C|GetLeftRight _asbp_fighter) 0.0) (Utilities|Enum|Equal(Enum) (Variables|/Game/Blueprints/Characters/BP_Fighter.BP_Fighter_C|GetStates _asbp_fighter) "NewEnumerator3"))
    (Utilities|FlowControl|Delay 0.2)
    (Actor|DestroyActor)))

(event EventTick
  (params (DeltaSeconds :type Float%20%28single-precision%29))
  (bind _returnvalue (Transformation|GetActorLocation))
  (bind (_x _y _z) (Math|Vector|BreakVector _returnvalue))
  (Utilities|FlowControl|Sequence
    (:then_0
      (CallFunction|Phase)
      (CallFunction|Leave)
      (if (> _z (Variables|Default|GetMoveZTo))
        (Transformation|SetActorLocation (Math|Interpolation|VInterpTo _returnvalue (Math|Vector|MakeVector _x _y (Variables|Default|GetMoveZTo)) DeltaSeconds 3.0) false false)))
    (:then_1
      (Utilities|FlowControl|Delay 5.0)
      (Actor|DestroyActor))))

(fn ConstructionScript
  (Collision|SetCollisionObjectType (Variables|Default|GetCylinder) "ECC_GameTraceChannel6"))

(fn Phase
  (bind _plats (Variables|Default|GetPlats))
  (Variables|Default|SetZpos (.Z (Math|Vector|BreakVector (Transformation|GetActorLocation))))
  (bind _outactors (Actor|GetAllActorsOfClass "/Game/Blueprints/Characters/BP_Fighter.BP_Fighter_C"))
  (for _array_element _outactors
    (if (> (Variables|/Game/Blueprints/Characters/BP_Fighter.BP_Fighter_C|GetFootZPos _array_element) (Variables|Default|GetZpos))
      (if (not (Variables|/Game/Blueprints/Characters/BP_Fighter.BP_Fighter_C|GetPlatPhaze _array_element))
        (Collision|SetCollisionResponsetoChannel (Variables|/Script/Engine.Character|GetCapsuleComponent _array_element) _plats "ECR_Block")
        (else
          (Collision|SetCollisionResponsetoChannel (Variables|/Script/Engine.Character|GetCapsuleComponent _array_element) _plats "ECR_Ignore" :!label _label)))
      (else
        (goto _label)))))