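; BP_sheild is a player's shield bubble, tinted by player number through a dynamic material instance.
; Tick scales the sphere to the HP fraction and, based on the parent's state, either shows it and decays HP or hides it and regenerates, paced by Delay.
; At zero HP, a DoOnce-guarded break launches the parent upward and dizzies them, re-arming during regeneration.
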(event Custom|Reset
  (bind _parent (Variables|Default|GetParent))
  ;[1 0.3191 0.6517 1 30] Shield Break
  (Utilities|FlowControl|DoOnce false) ; enters at Reset
)

(event Custom|ShieldBreak
  (bind _parent (Variables|Default|GetParent))
  ;[1 0.3191 0.6517 1 30] Shield Break
  (Utilities|FlowControl|DoOnce false
    (:Completed
      (Variables|/Game/Blueprints/Characters/BP_Fighter.BP_Fighter_C|SetLaunchValue _parent "0, 0,2000.000000")
      (Default|Launch _parent "0, 0,2000.000000" true true)
      (Variables|/Game/Blueprints/Characters/BP_Fighter.BP_Fighter_C|SetStates _parent "NewEnumerator14")
      (Variables|/Game/Blueprints/Characters/BP_Fighter.BP_Fighter_C|Setdizzied _parent true))))

(event EventTick
  (params (DeltaSeconds :type Float%20%28single-precision%29))
  (bind _sphere (Variables|Default|GetSphere))
  ;[0.4773 0.4503 1 1 30] Tick
  (Utilities|FlowControl|Sequence
    (:then_0
      ;;[0.5932 1 0.7301 1 30] Set Scale on %
      (bind _output_get (Variables|Default|SetPecent (/ (Math|Conversions|ToFloat(Integer) (Variables|Default|GetHP)) (Math|Conversions|ToFloat(Integer) (Variables|Default|GetMaxHP)))))
      (Transformation|SetWorldScale3D (Variables|Default|GetSphere) (Math|Conversions|ToVector(Float) (+ (Math|Interpolation|FInterpTo _output_get _output_get 0.0 (Variables|Default|GetRate)) 0.1))))
    (:then_1
      (if (Utilities|Enum|Equal(Enum) (Variables|/Game/Blueprints/Characters/BP_Fighter.BP_Fighter_C|GetStates (Variables|Default|GetParent)) "NewEnumerator12")
        ;;[0.8667 1 0.3083 1 30] set visible, decay HP
        (Rendering|SetVisibility _sphere true false)
        (if (> (Variables|Default|GetHP) 0)
          (Utilities|FlowControl|Delay (Variables|Default|GetRate))
          (Variables|Default|SetHP (- (Variables|Default|GetHP) (Variables|Default|GetDecay)))
          (else
            (CallFunction|ShieldBreak)))
        (else
          ;;[1 0.6524 0.3523 1 30] Set invisible, Regen HP
          (Rendering|SetVisibility _sphere false false)
          (if (< (Variables|Default|GetHP) (Variables|Default|GetMaxHP))
            (Utilities|FlowControl|Delay (Variables|Default|GetRate))
            (Variables|Default|SetHP (+ (Variables|Default|GetHP) (Variables|Default|GetRegen)))
            (CallFunction|Reset)))))))

(event EventBeginPlay
  (bind _material (Variables|Default|GetMaterial))
  ;[0.1198 1 0.9329 1 30] Set Color for each player
  (switch int (Variables|/Game/Blueprints/Characters/BP_Fighter.BP_Fighter_C|GetPlayerNo (Variables|Default|GetParent))
    (:0
      (Rendering|Material|SetVectorParameterValue _material "Color" "(R=0.070571,G=0.235724,B=0.583333,A=1.000000)" :!class /Script/Engine.MaterialInstanceDynamic))
    (:1
      (Rendering|Material|SetVectorParameterValue _material "Color" "(R=0.583333,G=0.006076,B=0.021175,A=1.000000)" :!class /Script/Engine.MaterialInstanceDynamic))
    (:2
      (Rendering|Material|SetVectorParameterValue _material "Color" "(R=0.000000,G=0.583333,B=0.102036,A=1.000000)" :!class /Script/Engine.MaterialInstanceDynamic))
    (:3
      (Rendering|Material|SetVectorParameterValue _material "Color" "(R=0.583333,G=0.539914,B=0.112894,A=1.000000)" :!class /Script/Engine.MaterialInstanceDynamic))))

(fn ConstructionScript
  (Variables|Default|SetHP (Variables|Default|GetMaxHP))
  (bind _returnvalue (Rendering|Material|CreateDynamicMaterialInstance (Variables|Default|GetSphere) 0 "/Game/Assets/Materials/Mat_sheild_Inst.Mat_sheild_Inst" :!class /Script/Engine.PrimitiveComponent))
  (Variables|Default|SetMaterial _returnvalue))