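; Base projectile Blueprint for a fighting game that damages any fighter except its owner on capsule overlap.
; Tick moves the mesh by fixed per-frame gravity and horizontal Y steps, unscaled by delta time, and calls EndLifeTime after a delay.
; Hits read damage, knockback and stun from DT_attackTable by AttackName, then play a sound.
; Most outcome events are empty hooks; reflection negates both speeds, though ZSpeed never drives movement.
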(event OnComponentBeginOverlap(Sphere)
  (params (OverlappedComponent :type Primitive%20Component%20Object%20Reference) (OtherActor :type Actor%20Object%20Reference) (OtherComp :type Primitive%20Component%20Object%20Reference) (OtherBodyIndex :type Integer) (bFromSweep :type Boolean) (SweepResult :type Hit%20Result%20Structure%20%28by%20ref%29))
  ;[0.4062 0.1037 0.1101 1 30] Overlap fighters
  (bind _asbp_fighter (Utilities|Casting|CastToBP_Fighter OtherActor))
  (if (and (== (Variables|/Script/Engine.Character|GetCapsuleComponent _asbp_fighter) OtherComp) (!= _asbp_fighter (Components|GetOwner)))
    (bind _returnvalue (Utilities|GetDataTableRow "/Game/Blueprints/AttackData/DT_attackTable.DT_attackTable" (Variables|Default|GetAttackName))
      (:then
        (Default|Hit _asbp_fighter "NewEnumerator0" (.Damage (Utilities|Struct|BreakST_AttacksStruct _returnvalue)) 0 (Math|Float|Truncate (.BaseKnock (Utilities|Struct|BreakST_AttacksStruct _returnvalue))) (.Scale (Utilities|Struct|BreakST_AttacksStruct _returnvalue)) (.Angle (Utilities|Struct|BreakST_AttacksStruct _returnvalue)) (.HitStop (Utilities|Struct|BreakST_AttacksStruct _returnvalue)) (.HitStun (Utilities|Struct|BreakST_AttacksStruct _returnvalue)) (Variables|Default|GetParent))
        (CallFunction|HitEvent)
        (CallFunction|PlayHitSound))
      (:RowNotFound
        (Development|PrintString "NoAttackFound" true true "(R=1.000000,G=0.000000,B=0.000000,A=1.000000)")))))

(event Custom|EndLifeTime
  ;[0.2165 0.5325 1 1 30] Even Calls
)

(event Custom|SetSpeed
  (params (YSpeed :type Float%20%28single-precision%29) (XSpeed :type Float%20%28single-precision%29))
  ;[0.2165 0.5325 1 1 30] Even Calls
  (Variables|Default|SetYSpeed YSpeed)
  (Variables|Default|SetZSpeed XSpeed))

(event Custom|PlayHitSound
  ;[1 1 1 1 30] HitSound
  (Audio|PlaySoundatLocation (Utilities|Array|Get(acopy) (Variables|Default|GetHitSound) (Variables|Default|GetsoundNo)) 0 (Variables|Default|GetLocation) "0, 0, 0" 1.0 1.0 0.0 0 0 0))

(event Custom|AbsorbedEvent
  ;[0.2165 0.5325 1 1 30] Even Calls
)

(event Custom|HitEvent
  ;[0.2165 0.5325 1 1 30] Even Calls
)

(event Custom|HitGroundEvent
  ;[0.2165 0.5325 1 1 30] Even Calls
)

(event Custom|HitWallEvent
  ;[0.2165 0.5325 1 1 30] Even Calls
)

(event Custom|ReflectedEvent
  ;[0.2165 0.5325 1 1 30] Even Calls
  (Variables|Default|SetYSpeed (* (Variables|Default|GetYSpeed) -1.0))
  (Variables|Default|SetZSpeed (* (Variables|Default|GetZSpeed) -1.0)))

(event EventTick
  (params (DeltaSeconds :type Float%20%28single-precision%29))
  ;[0.8249 1 0.2874 1 30] Tick
  (Variables|Default|SetLocation (Transformation|GetActorLocation))
  (Utilities|FlowControl|Sequence
    (:then_0
      (Utilities|FlowControl|Delay (Variables|Default|GetLifetIme))
      (CallFunction|EndLifeTime))
    (:then_1
      (CallFunction|FuncGravity)
      (CallFunction|MoveinDirection))))

(fn ConstructionScript)

(fn FuncGravity
  (bind _mesh (Variables|Default|GetMesh))
  (bind _returnvalue (Transformation|GetWorldLocation _mesh))
  (bind (_x _y _z) (Math|Vector|BreakVector _returnvalue))
  (Transformation|SetWorldLocation _mesh (Math|Vector|MakeVector _x _y (- _z (Variables|Default|GetGravity))) false false))

(fn MoveinDirection
  (bind _mesh (Variables|Default|GetMesh))
  (bind _mesh_2 (Variables|Default|GetMesh))
  (bind _returnvalue (Transformation|GetWorldLocation _mesh_2))
  (bind _returnvalue_2 (Transformation|GetWorldLocation _mesh))
  (bind (_x _y _z) (Math|Vector|BreakVector _returnvalue))
  (bind (_x_2 _y_2 _z_2) (Math|Vector|BreakVector _returnvalue_2))
  (switch Utilities|FlowControl|Switch|SwitchonEnum_faceing (Variables|Default|GetDirection)
    (:NewEnumerator0
      (Transformation|SetWorldLocation _mesh (Math|Vector|MakeVector _x_2 (+ _y_2 (Variables|Default|GetYSpeed)) _z_2) false false))
    (:NewEnumerator1
      (Transformation|SetWorldLocation _mesh_2 (Math|Vector|MakeVector _x (- _y (Variables|Default|GetYSpeed)) _z) false false))))