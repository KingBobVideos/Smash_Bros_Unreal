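; Placeholder pawn for each player in the platform fighter, replaced by the fighter chosen in the game instance.
; On BeginPlay it derives PlayerNo from the controller's display name, flags itself loaded in the game mode and removes itself for unused slots.
; Tick waits for GameState AllLoaded, then once spawns and possesses the character at the indexed BP_Spawn, updates the camera, adds HUD widgets and destroys itself.
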(event Custom|CreateCharacter
  (bind _playerno (Variables|Default|GetPlayerNo))
  ;[0.8235 0.6868 1 1 30] Create The playable characters
  (bind _outactors (Actor|GetAllActorsOfClass "/Game/Blueprints/LevelObjects/BP_Spawn.BP_Spawn_C"))
  (if (not (Utilities|Enum|Equal(Enum) (Utilities|Array|Get(acopy) (Variables|/Game/Blueprints/managers/GI_FighterGameInstance.GI_FighterGameInstance_C|GetPlayerCharacters (Variables|Default|GetGameInstance)) _playerno) "NewEnumerator1"))
    (CallFunction|SetCharacter (Math|Transform|MakeTransform (Transformation|GetActorLocation (Utilities|Array|Get(acopy) _outactors _playerno))))
    (bind _outactors_2 (Actor|GetAllActorsOfClass "/Game/Blueprints/LevelObjects/BP_camera.BP_camera_C"))
    (Default|UpdateCamera (Utilities|Array|Get(acopy) _outactors_2))
    (CallFunction|MakeHud)
    (Actor|DestroyActor)
    (else
      (Actor|DestroyActor))))

(event Custom|MakeHud
  (bind _returnvalue (Viewport|GetViewportSize))
  (bind _playerno (Variables|Default|GetPlayerNo))
  (bind (_x _y) (Math|Vector2D|BreakVector2D _returnvalue))
  ;[0.3958 0.2609 0.1506 1 40] MakeHUD
  (bind _returnvalue_2 (UserInterface|CreateWidget "/Game/Blueprints/Hud/InGame/HUD_CharacterInfo.HUD_CharacterInfo_C" 0 _playerno self))
  (UserInterface|Viewport|AddtoViewport _returnvalue_2 0)
  (Class|UserWidget|SetPositioninViewport _returnvalue_2 (Math|Vector2D|MakeVector2D (+ (* _playerno (/ _x (Math|Conversions|ToFloat(Integer) (Variables|/Game/Blueprints/managers/GI_FighterGameInstance.GI_FighterGameInstance_C|GetNumberOfPlayers (Variables|Default|GetGameInstance))))) 6e+01) (- _y 1.5e+02)) true)
  (bind _returnvalue_3 (UserInterface|CreateWidget "/Game/Blueprints/Hud/InGame/HUD_PlayerName.HUD_PlayerName_C" 0 _playerno self))
  (UserInterface|Viewport|AddtoViewport _returnvalue_3 0)
  (Class|UserWidget|SetPositioninViewport :self _returnvalue_3))

(event EventBeginPlay
  ;[0.349 0.349 0.349 1 30] Get GM, GI
  (Utilities|FlowControl|Delay 0.02)
  (bind _asgm_plat_fighter_gamemode (Utilities|Casting|CastToGM_PlatFighterGamemode (Game|GetGameMode))
    (:then
      (Variables|Default|SetGameMode _asgm_plat_fighter_gamemode))
    (:CastFailed
      _))
  (bind _asgs_fighter (Utilities|Casting|CastToGS_Fighter (Game|GetGameState))
    (:then
      (Variables|Default|Setgamestate _asgs_fighter))
    (:CastFailed
      _))
  (bind _asgi_fighter_game_instance (Utilities|Casting|CastToGI_FighterGameInstance (Game|GetGameInstance)))
  (bind _output_get (Variables|Default|SetGameInstance _asgi_fighter_game_instance))
  (CallFunction|SetPlayerNo)
  (if (> (Variables|Default|GetPlayerNo) (Variables|/Game/Blueprints/managers/GI_FighterGameInstance.GI_FighterGameInstance_C|GetNumberOfPlayers _output_get))
    (Actor|DestroyActor)))

(event EventTick
  (params (DeltaSeconds :type Float%20%28single-precision%29))
  (bind _gamestate (Variables|Default|Getgamestate))
  ;[0.6366 1 0.3728 1 30] Call Create Characters when all characters have loaded
  (Utilities|IsValid _gamestate
    (:Is%20Valid
      (if (Variables|/Game/Blueprints/managers/GS_Fighter.GS_Fighter_C|GetAllLoaded _gamestate)
        (Utilities|FlowControl|DoOnce false
          (:Completed
            (CallFunction|CreateCharacter)))))))

(fn ConstructionScript)

(fn SetPlayerNo
  ;[0.3866 0.4062 0.1583 1 40] Set The player ID no based on controller
  (Utilities|ElseBranch (or (Utilities|Enum|Equal(Enum) (Utilities|GetDisplayName (Pawn|GetController)) "BP_fighterController") (Utilities|Enum|Equal(Enum) (Utilities|GetDisplayName (Pawn|GetController)) "BP_fighterController_C_0")) (or (Utilities|Enum|Equal(Enum) (Utilities|GetDisplayName (Pawn|GetController)) "BP_fighterController1") (Utilities|Enum|Equal(Enum) (Utilities|GetDisplayName (Pawn|GetController)) "BP_fighterController_C_1")) (or (Utilities|Enum|Equal(Enum) (Utilities|GetDisplayName (Pawn|GetController)) "BP_fighterController2") (Utilities|Enum|Equal(Enum) (Utilities|GetDisplayName (Pawn|GetController)) "BP_fighterController_C_2"))
    (:If%20Con1
      (Variables|Default|SetPlayerNo 0))
    (:Else%20If%20Con2
      (Variables|Default|SetPlayerNo 1))
    (:Else%20If%20Con3
      (Variables|Default|SetPlayerNo 2))
    (:Else
      (Variables|Default|SetPlayerNo 3)))
  (Utilities|Array|SetArrayElem (Variables|/Game/Blueprints/managers/gamemodes/GM_PlatFighterGamemode.GM_PlatFighterGamemode_C|GetPlayerLoaded (Variables|Default|GetGameMode)) (Variables|Default|GetPlayerNo) true)
  (Rendering|Components|TextRender|SetText (Variables|Default|GetTextRender) (Utilities|Text|ToText(Integer) (Variables|Default|GetPlayerNo)))
  (if (Utilities|Enum|Equal(Enum) (Utilities|Array|Get(acopy) (Variables|/Game/Blueprints/managers/GI_FighterGameInstance.GI_FighterGameInstance_C|GetPlayerCharacters (Variables|Default|GetGameInstance)) (Variables|Default|GetPlayerNo)) "NewEnumerator1")
    (Actor|DestroyActor)))

(fn SetCharacter
  (params (Location :type Transform))
  ;[1 0 0.1804 1 40] This is where you set the characters that you play as
  (switch Utilities|FlowControl|Switch|SwitchonEnum_character (Utilities|Array|Get(acopy) (Variables|/Game/Blueprints/managers/GI_FighterGameInstance.GI_FighterGameInstance_C|GetPlayerCharacters (Variables|Default|GetGameInstance)) (Variables|Default|GetPlayerNo))
    (:NewEnumerator0
      (bind _returnvalue (Game|SpawnActorfromClass "/Game/Blueprints/Characters/BP_Fighter.BP_Fighter_C" Location "Undefined" (Pawn|GetController) (Variables|Default|GetPlayerNo) 0))
      (Pawn|Possess (Pawn|GetController) _returnvalue))
    (:NewEnumerator2
      (bind _returnvalue_2 (Game|SpawnActorfromClass "/Game/Blueprints/Characters/Fighters/PC_SwordFighter1.PC_SwordFighter1_C" Location "Undefined" (Pawn|GetController) (Variables|Default|GetPlayerNo) 0))
      (Pawn|Possess (Pawn|GetController) _returnvalue_2))
    (:NewEnumerator3
      (bind _returnvalue_3 (Game|SpawnActorfromClass "/Game/Blueprints/Characters/Fighters/PC_GunFighter.PC_GunFighter_C" Location "Undefined" (Pawn|GetController) (Variables|Default|GetPlayerNo) 0))
      (Pawn|Possess (Pawn|GetController) _returnvalue_3))
    (:NewEnumerator4
      (bind _returnvalue_4 (Game|SpawnActorfromClass "/Game/Blueprints/Characters/Fighters/PC_Hats.PC_Hats_C" Location "Undefined" (Pawn|GetController) (Variables|Default|GetPlayerNo) 0))
      (Pawn|Possess (Pawn|GetController) _returnvalue_4))
    (:NewEnumerator5
      (bind _returnvalue_5 (Game|SpawnActorfromClass "/Game/Blueprints/Characters/Fighters/PC_SwordFighter1.PC_SwordFighter1_C" Location "Undefined" (Pawn|GetController) (Variables|Default|GetPlayerNo) 0))
      (Pawn|Possess (Pawn|GetController) _returnvalue_5))
    (:NewEnumerator6
      (bind _returnvalue_6 (Game|SpawnActorfromClass "/Game/Blueprints/Characters/Fighters/PC_GunFighter.PC_GunFighter_C" Location "Undefined" (Pawn|GetController) (Variables|Default|GetPlayerNo) 0))
      (Pawn|Possess (Pawn|GetController) _returnvalue_6))
    (:NewEnumerator7
      (bind _returnvalue_7 (Game|SpawnActorfromClass "/Game/Blueprints/Characters/Fighters/PC_Hats.PC_Hats_C" Location "Undefined" (Pawn|GetController) (Variables|Default|GetPlayerNo) 0))
      (Pawn|Possess (Pawn|GetController) _returnvalue_7))))