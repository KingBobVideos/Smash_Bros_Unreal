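; Lobby manager actor for a fighter game that tracks player numbers, player count and ready states.
; On BeginPlay it derives the client number from the lobby character count, stores it in the game instance, and caches the lobby game mode on the host.
; Each tick, the host mirrors characters' ready flags into an array, and a ready instance calls ReadyUp on its matching character.
; Server and client update events store the player count and flag a list refresh.
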(event Custom|ServerUpdatePlayers
  (params (NumberOfPlayers :type Integer))
  ;[0.4846 1 0.8794 1 25] UpdatePlayers
  (bind _output_get (Variables|/Game/Blueprints/managers/GI_FighterGameInstance.GI_FighterGameInstance_C|SetNumberOfPlayers (Variables|Default|GetInstance) NumberOfPlayers))
  (Variables|Default|SetNumberOfPlayer _output_get)
  (Variables|Default|SetUpdateList true))

(event Custom|ClientUpdatePlayers
  (params (InputPin :type Integer))
  ;[0.4846 1 0.8794 1 25] UpdatePlayers
  (bind _output_get (Variables|/Game/Blueprints/managers/GI_FighterGameInstance.GI_FighterGameInstance_C|SetNumberOfPlayers (Variables|Default|GetInstance) InputPin))
  (Variables|Default|SetNumberOfPlayer _output_get)
  (Variables|Default|SetUpdateList true))

(event EventBeginPlay
  ;[1 0.4247 0.8843 1 25] Set Client No, Get GI, GM
  (Utilities|FlowControl|DoOnce false
    (:Completed
      (bind _outactors (Actor|GetAllActorsOfClass "/Game/Blueprints/Hud/Controllers/BP_LobyCharacter.BP_LobyCharacter_C"))
      (Variables|Default|SetClientNo (Utilities|Array|Length _outactors))
      (bind _asgi_fighter_game_instance (Utilities|Casting|CastToGI_FighterGameInstance (Game|GetGameInstance)))
      (bind _output_get (Variables|Default|SetInstance _asgi_fighter_game_instance))
      (Variables|/Game/Blueprints/managers/GI_FighterGameInstance.GI_FighterGameInstance_C|SetPlayerNumber _output_get (Variables|Default|GetClientNo))
      (if (Variables|/Game/Blueprints/managers/GI_FighterGameInstance.GI_FighterGameInstance_C|Gethost _output_get)
        (bind _asgm_lobby_mode (Utilities|Casting|CastToGM_LobbyMode (Game|GetGameMode)))
        (Variables|Default|SetgameMode _asgm_lobby_mode)))))

(event EventTick
  (params (DeltaSeconds :type Float%20%28single-precision%29))
  ;[0.3229 0.3229 0.3229 1 25] Tick
  (Utilities|FlowControl|Sequence
    (:then_0
      ;;[1 0.7368 0.6564] Is host
      (if (Variables|/Game/Blueprints/managers/GI_FighterGameInstance.GI_FighterGameInstance_C|Gethost (Variables|Default|GetInstance))
        (bind _outactors (Actor|GetAllActorsOfClass "/Game/Blueprints/Hud/Controllers/BP_LobyCharacter.BP_LobyCharacter_C"))
        (for (_array_element _array_index) _outactors
          (Utilities|Array|SetArrayElem (Variables|Default|GetReadyArray) _array_index (Variables|/Game/Blueprints/Hud/Controllers/BP_LobyCharacter.BP_LobyCharacter_C|GetReady _array_element) true))))
    (:then_1
      ;;[0.964 1 0.6827] Is Ready?
      (if (Variables|/Game/Blueprints/managers/GI_FighterGameInstance.GI_FighterGameInstance_C|GetReady (Variables|Default|GetInstance))
        (bind _outactors_2 (Actor|GetAllActorsOfClass "/Game/Blueprints/Hud/Controllers/BP_LobyCharacter.BP_LobyCharacter_C"))
        (for _array_element_2 _outactors_2
          (if (== (Variables|/Game/Blueprints/Hud/Controllers/BP_LobyCharacter.BP_LobyCharacter_C|GetPlayerNo _array_element_2) (Variables|Default|GetClientNo))
            (Default|ReadyUp _array_element_2 (Variables|/Game/Blueprints/Hud/Controllers/BP_LobyCharacter.BP_LobyCharacter_C|GetPlayerNo _array_element_2))))))))

(fn ConstructionScript)