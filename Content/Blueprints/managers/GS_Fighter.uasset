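; Game state for the platform fighter that runs match rules for Stock and Time modes and tracks when all players have loaded.
; Tick updates the countdown and Elims-minus-Falls scores, ending the match at one player alive or when time expires.
; Player deaths update alive and placement data in the game instance, from which the winner is set.
; Match end slows global time, then opens VictoryScreen, using server travel when online.
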(event Custom|GameEnd
  ;[1 0.8394 0.1886 1 30] End Game
  (Utilities|FlowControl|DoOnce false
    (:Completed
      (CallFunction|SetWinner)
      (CallFunction|EndGameServer)
      (if (Variables|/Game/Blueprints/managers/GI_FighterGameInstance.GI_FighterGameInstance_C|GetOnline (Variables|Default|GetInstance))
        (CallFunction|EndGameClients)))))

(event Custom|EndGameServer
  ;[1 0.8394 0.1886 1 30] End Game
  (Variables|/Game/Blueprints/managers/GI_FighterGameInstance.GI_FighterGameInstance_C|SetEndGame (Variables|Default|GetInstance) true)
  (Utilities|FlowControl|Delay 0.01)
  (Utilities|Time|SetGlobalTimeDilation (Math|Interpolation|FInterpTo (Class|GameplayStatics|GetGlobalTimeDilation) 0.1 (Variables|Default|GetDelta) 1.0))
  (Utilities|FlowControl|Delay 2.0)
  (if (Variables|/Game/Blueprints/managers/GI_FighterGameInstance.GI_FighterGameInstance_C|GetOnline (Variables|Default|GetInstance))
    (Default|ServerTravle (Variables|Default|GetInstance) "VictoryScreen")
    (else
      (Game|OpenLevel(byName) "VictoryScreen"))))

(event Custom|OnlineLoaded
  ;[1 0.581 0.966 1 30] All Online Players Have Loaded
  (Utilities|FlowControl|Delay 0.01)
  (for _index (range 0 (Variables|/Game/Blueprints/managers/GI_FighterGameInstance.GI_FighterGameInstance_C|GetNumberOfPlayers (Variables|Default|GetInstance)))
    (Utilities|Array|SetArrayElem (Variables|Default|GetPlayerLoaded) _index false true)))

(event Custom|PlayerDeath
  (params (PlayerNo :type Integer))
  (CallFunction|FuncPlayerDeath PlayerNo))

(event Custom|EndGameClients
  ;[1 0.8394 0.1886 1 30] End Game
  (Variables|/Game/Blueprints/managers/GI_FighterGameInstance.GI_FighterGameInstance_C|SetEndGame (Variables|Default|GetInstance) true)
  (Utilities|FlowControl|Delay 0.01)
  (Utilities|Time|SetGlobalTimeDilation (Math|Interpolation|FInterpTo (Class|GameplayStatics|GetGlobalTimeDilation) 0.1 (Variables|Default|GetDelta) 1.0)))

(event EventBeginPlay
  ;[0.5535 1 0.2465 1 30] BeginPlay
  (bind _asgi_fighter_game_instance (Utilities|Casting|CastToGI_FighterGameInstance (Game|GetGameInstance)))
  (Variables|Default|SetInstance _asgi_fighter_game_instance)
  (bind _asgm_plat_fighter_gamemode (Utilities|Casting|CastToGM_PlatFighterGamemode (Game|GetGameMode)))
  (Variables|Default|SetGameMode _asgm_plat_fighter_gamemode)
  (CallFunction|OnlineLoaded)
  (if (Utilities|Enum|Equal(Enum) (Variables|Default|GetMode) "NewEnumerator1")
    (Variables|Default|SetTimer true)
    (else
      (Variables|Default|SetTimer false))))

(event EventTick
  (params (DeltaSeconds :type Float%20%28single-precision%29))
  ;[1 1 1 1 30] Tick
  (Variables|Default|SetDelta DeltaSeconds)
  (Utilities|FlowControl|Sequence
    (:then_0
      (CallFunction|FuncEndgame)
      (CallFunction|FuncTimer))
    (:then_1
      (if (not (Utilities|Array|ContainsItem (Variables|Default|GetPlayerLoaded) false))
        (Variables|Default|SetAllLoaded true)))))

(fn ConstructionScript)

(fn FuncTimer
  (if (Variables|Default|GetTimer)
    (CallFunction|TimerPositions)
    (Utilities|FlowControl|Sequence
      (:then_0
        (bind _output_get (Variables|Default|SetSeconds (- (Variables|Default|GetSeconds) (Variables|Default|GetDelta))))
        (if (> (Math|Float|Round _output_get) 9)
          (Variables|Default|SetTimerText (Utilities|String|Append (Utilities|String|Append (Utilities|String|ToString(Integer) (Variables|Default|GetMin)) ":") (Utilities|String|ToString(Integer) (Math|Float|Round _output_get))))
          (else
            (Variables|Default|SetTimerText (Utilities|String|Append (Utilities|String|Append (Utilities|String|Append (Utilities|String|ToString(Integer) (Variables|Default|GetMin)) ":") "0") (Utilities|String|ToString(Integer) (Math|Float|Round _output_get)))))))
      (:then_1
        (if (<= (Variables|Default|GetSeconds) 0.0)
          (Variables|Default|SetSeconds 6e+01)
          (Math|Integer|DecrementInt (Variables|Default|GetMin)))))))

(fn FuncEndgame
  (switch Utilities|FlowControl|Switch|SwitchonEnum_InGameModes (Variables|Default|GetMode)
    (:NewEnumerator0
      ;[1 1 1] StockMode
      (if (== (Variables|/Game/Blueprints/managers/GI_FighterGameInstance.GI_FighterGameInstance_C|GetPlayersAlive (Variables|Default|GetInstance)) 1)
        (Utilities|FlowControl|DoOnce false :!label _label
          (:Completed
            (CallFunction|GameEnd)))
        (else
          (goto _label Reset))))
    (:NewEnumerator1
      ;[1 1 1] TimeMode
      (if (< (Variables|Default|GetMin) 0)
        (Utilities|FlowControl|DoOnce false :!label _label_2
          (:Completed
            (Variables|Default|SetTimer false)
            (CallFunction|GameEnd)))
        (else
          (goto _label_2 Reset))))))

(fn TimerPositions
  (for _index (range 0 (Variables|Default|GetPlayersAlive))
    (Utilities|Array|SetArrayElem (Variables|/Game/Blueprints/managers/GI_FighterGameInstance.GI_FighterGameInstance_C|GetScore (Variables|Default|GetInstance)) _index (- (Utilities|Array|Get(acopy) (Variables|Default|GetElims) _index) (Utilities|Array|Get(acopy) (Variables|Default|GetFalls) _index)) true)))

(fn SetWinner
  (bind _instance (Variables|Default|GetInstance))
  (bind _playerpositions (Variables|/Game/Blueprints/managers/GI_FighterGameInstance.GI_FighterGameInstance_C|GetPlayerPositions _instance))
  (for (_array_element _array_index) (Variables|/Game/Blueprints/managers/GI_FighterGameInstance.GI_FighterGameInstance_C|GetAliveArray (Variables|Default|GetInstance))
    (if (Math|Boolean|Equal(Boolean) _array_element true)
      (bind _output_get (Variables|/Game/Blueprints/managers/GI_FighterGameInstance.GI_FighterGameInstance_C|SetWinner _instance _array_index))
      (Utilities|Array|Insert _playerpositions 0 _output_get)
      (Utilities|Array|SetArrayElem _playerpositions 0 _output_get true))))

(fn FuncPlayerDeath
  (params (PlayerNo :type Integer))
  (bind _instance (Variables|Default|GetInstance))
  (Utilities|Array|SetArrayElem (Variables|/Game/Blueprints/managers/GI_FighterGameInstance.GI_FighterGameInstance_C|GetAliveArray _instance) PlayerNo false)
  (Utilities|Array|Insert (Variables|/Game/Blueprints/managers/GI_FighterGameInstance.GI_FighterGameInstance_C|GetPlayerPositions _instance) PlayerNo)
  (Variables|/Game/Blueprints/managers/GI_FighterGameInstance.GI_FighterGameInstance_C|SetPlayersAlive _instance (- (Variables|/Game/Blueprints/managers/GI_FighterGameInstance.GI_FighterGameInstance_C|GetPlayersAlive _instance) 1)))