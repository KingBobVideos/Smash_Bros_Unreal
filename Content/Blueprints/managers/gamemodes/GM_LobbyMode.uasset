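; GM_LobbyMode is the lobby game mode that starts the multiplayer match once everyone is ready.
; On BeginPlay it caches the fighter GameInstance and the lobby manager actor, then pushes the player count to that manager shortly after each PostLogin.
; Tick polls the manager's ready array and, when all are ready and the GameInstance counts multiple players, triggers a one-time server travel to ConflictZone.
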(event Custom|StartMatch
  ;[0.7396 1 0.4792 1 25] Travle to map
  (Development|ExecuteConsoleCommand "servertravel ConflictZone" (Game|GetPlayerController 0)))

(event EventBeginPlay
  ;[0.986 0.5993 1 1 25] Set Game instance
  (bind _asgi_fighter_game_instance (Utilities|Casting|CastToGI_FighterGameInstance (Game|GetGameInstance)))
  (Variables|Default|SetGameInstance _asgi_fighter_game_instance)
  (bind _outactors (Actor|GetAllActorsOfClass "/Game/Blueprints/managers/BP_lobbyMannager.BP_lobbyMannager_C"))
  (Variables|Default|SetManager (Utilities|Array|Get(acopy) _outactors)))

(event EventTick
  (params (DeltaSeconds :type Float%20%28single-precision%29))
  ;[1 0.7458 0.4077 1 25] Comment
  (if (and (not (Utilities|Array|ContainsItem (Variables|/Game/Blueprints/managers/BP_lobbyMannager.BP_lobbyMannager_C|GetReadyArray (Variables|Default|GetManager)) false)) (> (Variables|/Game/Blueprints/managers/GI_FighterGameInstance.GI_FighterGameInstance_C|GetNumberOfPlayers (Variables|Default|GetGameInstance)) 1))
    (Utilities|FlowControl|DoOnce false
      (:Completed
        (CallFunction|StartMatch)))))

(event EventPostLogin
  (params (NewPlayer :type Player%20Controller%20Object%20Reference))
  (bind _manager (Variables|Default|GetManager))
  ;[1 0.6131 0.5932 1 25] PlayerConnect
  (Utilities|FlowControl|Delay 0.01)
  (bind _returnvalue (Class|GameModeBase|GetNumPlayers (Game|GetGameMode)))
  (Default|ServerUpdatePlayers _manager _returnvalue)
  (Default|ClientUpdatePlayers _manager _returnvalue))

(fn ConstructionScript)