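; Menu game mode for a fighting game, handling main menu, character select and map select navigation and loading the chosen level.
; Input events branch on the menu type cached from GI_FighterGameInstance, stepping a menu index or per-player row and column arrays with click sounds.
; MenuAction locks a player's character pick, freezing their cursor.
; GameStart opens the selected map; Random's RandomInteger(2) never reaches BattlePlace, and MenuStart is an empty switch.
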(event Custom|selectsound
  ;[0.5272 1 0.3558 1 30] Play Sounds
  (Audio|PlaySound2D "/Game/Assets/Sounds/Menu/SC_menu_select_Cue.SC_menu_select_Cue" 1.0 1.0 0.0 0 0))

(event Custom|GameStart
  ;[1 0.6387 0.2958 1 30] Load Map
  (Variables|Default|SetStart true)
  (switch Utilities|FlowControl|Switch|SwitchonEnum_Maps (Variables|Default|GetMap)
    (:NewEnumerator1
      (Game|OpenLevel(byName) "ConflictZone" :!label _label))
    (:NewEnumerator0
      (Game|OpenLevel(byName) "Concluding_Ground" :!label _label_2))
    (:NewEnumerator9
      (Game|OpenLevel(byName) "BattlePlace" :!label _label_3))
    (:NewEnumerator8
      (switch int (Math|Random|RandomInteger 2)
        (:0
          (goto _label))
        (:1
          (goto _label_2))
        (:2
          (goto _label_3))))))

(event Custom|RightEvent
  (params (PlayerNo :type Integer))
  ;[0.4823 0.3275 1 1 30] Right Direction
  (switch Utilities|FlowControl|Switch|SwitchonEnum_menus (Variables|Default|GetMenus)
    (:NewEnumerator2
      (if (not (Utilities|Array|Get(acopy) (Variables|Player|GetPlayerSelected) PlayerNo))
        (Utilities|AddtoArray (Variables|Default|GetCols) PlayerNo 1 :!label _label
          (:%20
            (CallFunction|MenuClickSound)))))
    (:NewEnumerator3
      (goto _label))))

(event Custom|UpEvent
  (params (PlayerNo :type Integer))
  ;[0.3979 1 0.6978 1 30] Press Up
  (switch Utilities|FlowControl|Switch|SwitchonEnum_menus (Variables|Default|GetMenus)
    (:NewEnumerator0
      (Variables|Default|SetMenueNumber (- (Variables|Default|GetMenueNumber) 1))
      (CallFunction|MenuClickSound))
    (:NewEnumerator2
      (if (not (Utilities|Array|Get(acopy) (Variables|Player|GetPlayerSelected) PlayerNo))
        (Utilities|SubtractfromArray (Variables|Default|GetRows) PlayerNo 1 :!label _label
          (:%20
            (CallFunction|MenuClickSound)))))
    (:NewEnumerator3
      (goto _label))))

(event Custom|DownEvent
  (params (PlayerNo :type Integer))
  ;[0.9354 1 0.3379 1 30] Press Down
  (switch Utilities|FlowControl|Switch|SwitchonEnum_menus (Variables|Default|GetMenus)
    (:NewEnumerator0
      (Variables|Default|SetMenueNumber (+ (Variables|Default|GetMenueNumber) 1))
      (CallFunction|MenuClickSound))
    (:NewEnumerator2
      (if (not (Utilities|Array|Get(acopy) (Variables|Player|GetPlayerSelected) PlayerNo))
        (Utilities|AddtoArray (Variables|Default|GetRows) PlayerNo 1 :!label _label
          (:%20
            (CallFunction|MenuClickSound)))))
    (:NewEnumerator3
      (goto _label))))

(event Custom|MenuStart
  ;[0.3733 0.776 1 1 30] Start Action
  (switch Utilities|FlowControl|Switch|SwitchonEnum_menus (Variables|Default|GetMenus)))

(event Custom|LeftEvent
  (params (PlayerNo :type Integer))
  ;[1 0.4683 0.4882 1 30] Left Direction
  (switch Utilities|FlowControl|Switch|SwitchonEnum_menus (Variables|Default|GetMenus)
    (:NewEnumerator2
      (if (not (Utilities|Array|Get(acopy) (Variables|Player|GetPlayerSelected) PlayerNo))
        (Utilities|SubtractfromArray (Variables|Default|GetCols) PlayerNo 1 :!label _label
          (:%20
            (CallFunction|MenuClickSound)))))
    (:NewEnumerator3
      (goto _label))))

(event Custom|MenuClickSound
  ;[0.5272 1 0.3558 1 30] Play Sounds
  (Audio|PlaySound2D "/Game/Assets/Sounds/Menu/SC_menu_click_Cue.SC_menu_click_Cue" 1.0 1.0 0.0 0 0))

(event Custom|MenuAction
  (params (Player :type Integer))
  (bind _playerselected (Variables|Player|GetPlayerSelected))
  ;[1 0.4689 0.8954 1 30] Select Action
  (switch Utilities|FlowControl|Switch|SwitchonEnum_menus (Variables|Default|GetMenus)
    (:NewEnumerator2
      (if (not (Utilities|Array|Get(acopy) _playerselected Player))
        (Utilities|Array|SetArrayElem _playerselected Player true)))))

(event EventBeginPlay
  ;[0.4983 0.9602 1 1 30] Comment
  (bind _asgi_fighter_game_instance (Utilities|Casting|CastToGI_FighterGameInstance (Game|GetGameInstance)))
  (bind _output_get (Variables|Default|SetGameInstance _asgi_fighter_game_instance))
  (Variables|Default|SetGameMode (Variables|/Game/Blueprints/managers/GI_FighterGameInstance.GI_FighterGameInstance_C|GetMainMode _output_get))
  (Variables|Default|SetMenus (Variables|/Game/Blueprints/managers/GI_FighterGameInstance.GI_FighterGameInstance_C|GetMenus _output_get)))

(fn ConstructionScript)