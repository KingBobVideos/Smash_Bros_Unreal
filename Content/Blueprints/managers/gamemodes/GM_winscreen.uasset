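; Game mode for the win screen that returns the fighter game to the menus.
; BeginPlay caches the fighter game instance.
; PressStartEvent, gated by the CanProg flag, removes the extra local players along with their pawns, using the instance's player count.
; It also resets the alive-player count and end-game flag on the game instance and opens the menus level.
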(event Custom|PressStartEvent
  (bind _gameinstance (Variables|Default|GetGameInstance))
  ;[1 1 1] Go back to menues
  (if (Variables|Default|GetCanProg)
    (for _index (range 1 (Variables|/Game/Blueprints/managers/GI_FighterGameInstance.GI_FighterGameInstance_C|GetNumberOfPlayers _gameinstance))
      (Class|GameplayStatics|RemovePlayer (Game|GetPlayerController _index) true))
    (Variables|/Game/Blueprints/managers/GI_FighterGameInstance.GI_FighterGameInstance_C|SetPlayersAlive _gameinstance 4)
    (Game|OpenLevel(byName) "menus")
    (Variables|/Game/Blueprints/managers/GI_FighterGameInstance.GI_FighterGameInstance_C|SetEndGame (Variables|Default|GetGameInstance) false)))

(event EventBeginPlay
  (bind _asgi_fighter_game_instance (Utilities|Casting|CastToGI_FighterGameInstance (Game|GetGameInstance)))
  (Variables|Default|SetGameInstance _asgi_fighter_game_instance))

(fn ConstructionScript)